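; BP_Slump is a block actor with five plane trigger zones, called sustrate zones.
; On BeginPlay it runs the parent logic, then registers each plane in the SustrateZones map with a float weight, the fifth weighted higher than the rest.
; Each plane's begin-overlap event forwards the overlapped component and other actor to TriggerSustrateZones, whose logic is defined outside this graph.
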(event OnComponentBeginOverlap(PlaneSustrateZone1)
  (params (OverlappedComponent :type Primitive%20Component%20Object%20Reference) (OtherActor :type Actor%20Object%20Reference) (OtherComp :type Primitive%20Component%20Object%20Reference) (OtherBodyIndex :type Integer) (bFromSweep :type Boolean) (SweepResult :type Hit%20Result%20Structure%20%28by%20ref%29))
  ;[1 1 1] Events of overlapping
  (CallFunction|TriggerSustrateZones OverlappedComponent OtherActor))

(event OnComponentBeginOverlap(PlaneSustrateZone2)
  (params (OverlappedComponent :type Primitive%20Component%20Object%20Reference) (OtherActor :type Actor%20Object%20Reference) (OtherComp :type Primitive%20Component%20Object%20Reference) (OtherBodyIndex :type Integer) (bFromSweep :type Boolean) (SweepResult :type Hit%20Result%20Structure%20%28by%20ref%29))
  ;[1 1 1] Events of overlapping
  (CallFunction|TriggerSustrateZones OverlappedComponent OtherActor))

(event OnComponentBeginOverlap(PlaneSustrateZone3)
  (params (OverlappedComponent :type Primitive%20Component%20Object%20Reference) (OtherActor :type Actor%20Object%20Reference) (OtherComp :type Primitive%20Component%20Object%20Reference) (OtherBodyIndex :type Integer) (bFromSweep :type Boolean) (SweepResult :type Hit%20Result%20Structure%20%28by%20ref%29))
  ;[1 1 1] Events of overlapping
  (CallFunction|TriggerSustrateZones OverlappedComponent OtherActor))

(event OnComponentBeginOverlap(PlaneSustrateZone4)
  (params (OverlappedComponent :type Primitive%20Component%20Object%20Reference) (OtherActor :type Actor%20Object%20Reference) (OtherComp :type Primitive%20Component%20Object%20Reference) (OtherBodyIndex :type Integer) (bFromSweep :type Boolean) (SweepResult :type Hit%20Result%20Structure%20%28by%20ref%29))
  ;[1 1 1] Events of overlapping
  (CallFunction|TriggerSustrateZones OverlappedComponent OtherActor))

(event OnComponentBeginOverlap(PlaneSustrateZone5)
  (params (OverlappedComponent :type Primitive%20Component%20Object%20Reference) (OtherActor :type Actor%20Object%20Reference) (OtherComp :type Primitive%20Component%20Object%20Reference) (OtherBodyIndex :type Integer) (bFromSweep :type Boolean) (SweepResult :type Hit%20Result%20Structure%20%28by%20ref%29))
  ;[1 1 1] Events of overlapping
  (CallFunction|TriggerSustrateZones OverlappedComponent OtherActor))

(event EventBeginPlay
  (|CallParentFunction)
  ;[1 1 1] Add sustrate zones at Map
  (Utilities|Map|Add (Variables|Default|GetSustrateZones) (Variables|Default|GetPlaneSustrateZone1) 0.2)
  (Utilities|Map|Add (Variables|Default|GetSustrateZones) (Variables|Default|GetPlaneSustrateZone2) 0.2)
  (Utilities|Map|Add (Variables|Default|GetSustrateZones) (Variables|Default|GetPlaneSustrateZone3) 0.2)
  (Utilities|Map|Add (Variables|Default|GetSustrateZones) (Variables|Default|GetPlaneSustrateZone4) 0.2)
  (Utilities|Map|Add (Variables|Default|GetSustrateZones) (Variables|Default|GetPlaneSustrateZone5) 1.0))

(event Collision|EventActorBeginOverlap
  (params (OtherActor :type Actor%20Object%20Reference)))

(event EventTick
  (params (DeltaSeconds :type Float%20%28single-precision%29)))

(fn ConstructionScript
  (|CallParentFunction))