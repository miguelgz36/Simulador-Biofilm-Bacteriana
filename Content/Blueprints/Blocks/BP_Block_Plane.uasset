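; BP_Block_Plane is a block actor that acts as a nutrient-bearing surface for bacteria.
; When an actor enters its PlaneSustrateZone component, the overlap event casts it to BP_Bacteria and ignores anything else.
; BacteriaBeginOverlapSurface then passes the plane's available nutrients to that bacteria through SetAvailableNutrient.
; The file has no end-overlap handling, and its construction script only calls the parent.
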(event OnComponentBeginOverlap(PlaneSustrateZone)
  (params (OverlappedComponent :type Primitive%20Component%20Object%20Reference) (OtherActor :type Actor%20Object%20Reference) (OtherComp :type Primitive%20Component%20Object%20Reference) (OtherBodyIndex :type Integer) (bFromSweep :type Boolean) (SweepResult :type Hit%20Result%20Structure%20%28by%20ref%29))
  ;[1 1 1] Set available nutrients of bacteria that begin overlap surface
  (bind _asbp_bacteria (Utilities|Casting|CastToBP_Bacteria OtherActor))
  (CallFunction|BacteriaBeginOverlapSurface _asbp_bacteria (Variables|AvailabeNutrients|GetPlaneAvailableNutrients)))

(event EventBeginPlay
  (|CallParentFunction) ; This node is disabled and will not be called.\nDrag off pins to build functionality.
)

(event Collision|EventActorBeginOverlap
  (params (OtherActor :type Actor%20Object%20Reference))
  (|CallParentFunction OtherActor) ; This node is disabled and will not be called.\nDrag off pins to build functionality.
)

(event EventTick
  (params (DeltaSeconds :type Float%20%28single-precision%29))
  (|CallParentFunction DeltaSeconds) ; This node is disabled and will not be called.\nDrag off pins to build functionality.
)

(fn ConstructionScript
  (|CallParentFunction))

(fn BacteriaBeginOverlapSurface
  (params (Bacteria :type BP%20Bacteria%20Object%20Reference) (AvailableNutrients :type Float%20%28single-precision%29))
  (Default|SetAvailableNutrient Bacteria AvailableNutrients))