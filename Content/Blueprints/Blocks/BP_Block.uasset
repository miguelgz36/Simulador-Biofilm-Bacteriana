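; BP_Block is a block actor that tracks substrate nutrients per surface zone for bacteria.
; A map keyed by static mesh component stores each zone's nutrient value, which AddSustrateNutrients increments.
; TriggerSustrateZones handles zone overlaps: bacteria receive that zone's available nutrients, while substrate balls receive zone and block references and have their tick enabled.
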(event EventBeginPlay)

(event Collision|EventActorBeginOverlap
  (params (OtherActor :type Actor%20Object%20Reference)))

(event EventTick
  (params (DeltaSeconds :type Float%20%28single-precision%29)))

(fn ConstructionScript)

(fn AddSustrateNutrients
  (params (NewValue :type Float%20%28single-precision%29%20%28by%20ref%29) (SustrateZone :type Static%20Mesh%20Component%20Object%20Reference%20%28by%20ref%29))
  (bind _sustratezones (Variables|Surface|GetSustrateZones))
  (Utilities|Map|Add _sustratezones SustrateZone (+ NewValue (.Value (Utilities|Map|Find _sustratezones SustrateZone))))
  (return))

(fn TriggerSustrateZones
  (params (OverlappedComponent :type Primitive%20Component%20Object%20Reference%20%28by%20ref%29) (OtherActor :type Actor%20Object%20Reference%20%28by%20ref%29))
  (bind _asstatic_mesh_component (Utilities|Casting|CastToStaticMeshComponent OverlappedComponent))
  ;[1 1 1] Set available nutrients of bacteria that begin overlap surface
  (bind _asbp_bacteria (Utilities|Casting|CastToBP_Bacteria OtherActor)
    (:then
      (Default|SetAvailableNutrient _asbp_bacteria (.Value (Utilities|Map|Find (Variables|Surface|GetSustrateZones) _asstatic_mesh_component))))
    (:CastFailed
      ;[1 1 1] Set nutrients of sustrate zone when a sustrate ball begin overlap it
      (bind _asbp_sustrate_ball (Utilities|Casting|CastToBP_SustrateBall OtherActor))
      (Variables|/Game/Blueprints/PreSimulation/BP_SustrateBall.BP_SustrateBall_C|SetSustrateZone _asbp_sustrate_ball _asstatic_mesh_component)
      (Variables|/Game/Blueprints/PreSimulation/BP_SustrateBall.BP_SustrateBall_C|SetBlock _asbp_sustrate_ball self)
      (Actor|Tick|SetActorTickEnabled _asbp_sustrate_ball true)))
  (return))