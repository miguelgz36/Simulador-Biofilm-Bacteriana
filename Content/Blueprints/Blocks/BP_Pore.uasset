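; BP_Pore is a pore block that registers five substrate zone planes for overlap detection.
; On BeginPlay, after the parent's setup, it fills the SustrateZones map, pairing each plane with a float weight that is higher for the fifth zone.
; Each plane's begin-overlap event forwards the plane and the overlapping actor to a shared TriggerSustrateZones function, whose logic lies outside this graph.
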(event OnComponentBeginOverlap(PlaneSustrateZone1)
  (params (OverlappedComponent :type Primitive%20Component%20Object%20Reference) (OtherActor :type Actor%20Object%20Reference) (OtherComp :type Primitive%20Component%20Object%20Reference) (OtherBodyIndex :type Integer) (bFromSweep :type Boolean) (SweepResult :type Hit%20Result%20Structure%20%28by%20ref%29))
  (CallFunction|TriggerSustrateZones OverlappedComponent OtherActor))

(event OnComponentBeginOverlap(PlaneSustrateZone2)
  (params (OverlappedComponent :type Primitive%20Component%20Object%20Reference) (OtherActor :type Actor%20Object%20Reference) (OtherComp :type Primitive%20Component%20Object%20Reference) (OtherBodyIndex :type Integer) (bFromSweep :type Boolean) (SweepResult :type Hit%20Result%20Structure%20%28by%20ref%29))
  (CallFunction|TriggerSustrateZones OverlappedComponent OtherActor))

(event OnComponentBeginOverlap(PlaneSustrateZone3)
  (params (OverlappedComponent :type Primitive%20Component%20Object%20Reference) (OtherActor :type Actor%20Object%20Reference) (OtherComp :type Primitive%20Component%20Object%20Reference) (OtherBodyIndex :type Integer) (bFromSweep :type Boolean) (SweepResult :type Hit%20Result%20Structure%20%28by%20ref%29))
  (CallFunction|TriggerSustrateZones OverlappedComponent OtherActor))

(event OnComponentBeginOverlap(PlaneSustrateZone4)
  (params (OverlappedComponent :type Primitive%20Component%20Object%20Reference) (OtherActor :type Actor%20Object%20Reference) (OtherComp :type Primitive%20Component%20Object%20Reference) (OtherBodyIndex :type Integer) (bFromSweep :type Boolean) (SweepResult :type Hit%20Result%20Structure%20%28by%20ref%29))
  (CallFunction|TriggerSustrateZones OverlappedComponent OtherActor))

(event OnComponentBeginOverlap(PlaneSustrateZone5)
  (params (OverlappedComponent :type Primitive%20Component%20Object%20Reference) (OtherActor :type Actor%20Object%20Reference) (OtherComp :type Primitive%20Component%20Object%20Reference) (OtherBodyIndex :type Integer) (bFromSweep :type Boolean) (SweepResult :type Hit%20Result%20Structure%20%28by%20ref%29))
  (CallFunction|TriggerSustrateZones OverlappedComponent OtherActor))

(event EventBeginPlay
  (|CallParentFunction)
  (Utilities|Map|Add (Variables|Default|GetSustrateZones) (Variables|Default|GetPlaneSustrateZone1) 0.3)
  (Utilities|Map|Add (Variables|Default|GetSustrateZones) (Variables|Default|GetPlaneSustrateZone2) 0.3)
  (Utilities|Map|Add (Variables|Default|GetSustrateZones) (Variables|Default|GetPlaneSustrateZone3) 0.3)
  (Utilities|Map|Add (Variables|Default|GetSustrateZones) (Variables|Default|GetPlaneSustrateZone4) 0.3)
  (Utilities|Map|Add (Variables|Default|GetSustrateZones) (Variables|Default|GetPlaneSustrateZone5) 0.7))

(event Collision|EventActorBeginOverlap
  (params (OtherActor :type Actor%20Object%20Reference))
  (|CallParentFunction OtherActor) ; This node is disabled and will not be called.\nDrag off pins to build functionality.
)

(event EventTick
  (params (DeltaSeconds :type Float%20%28single-precision%29))
  (|CallParentFunction DeltaSeconds) ; This node is disabled and will not be called.\nDrag off pins to build functionality.
)

(fn ConstructionScript
  (|CallParentFunction))