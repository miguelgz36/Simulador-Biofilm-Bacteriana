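; Player-controlled camera character for a simulator, moved by keyboard, mouse and on-screen HUD controls.
; BeginPlay creates the HUD_In_Execution widget and binds its events for movement, zoom, pause, resume and quit.
; Mouse drags rotate the view, while wheel and slider zoom by changing spring arm length.
; Key flags gate keyboard movement; two looping timers detect both mouse buttons held, which blocks look and keyboard movement and pans vertically and sideways instead.
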(event Custom|OnZoomSliderChanged
  (params (NewValue :type Float%20%28single-precision%29))
  ;[1 1 1] Zoom In and Zoom Out With Slider
  (CallFunction|ZoomGui NewValue))

(event Custom|BothMouses
  ;[1 1 1] Setup Both Mouse Buttons
  (CallFunction|SetupBothMouses))

(event Custom|OnClickedButtonDown
  ;[1 1 1] Move Backward with Button
  (CallFunction|MoveForwardGui -1.0))

(event Custom|OnClickedButtonResume
  ;[1 1 1] Resume Simulation with Button
  (CallFunction|UnPauseSimulation))

(event Custom|OnClickedButtonQuit
  ;[1 1 1] Quit Simulation with Button
  (CallFunction|QuitSimulation))

(event Custom|BothMousesCheck
  ;[1 1 1] Setup Both Mouse Buttons
  (CallFunction|SetupBothMousesCheck))

(event Custom|OnClickedButtonRight
  ;[1 1 1] Move Right with Button
  (CallFunction|MoveRightGui 1.0))

(event Custom|OnClickedButtonPause
  ;[1 1 1] Pause Simulation with Button
  (CallFunction|PauseSimulation))

(event Custom|OnClickedButtonLeft
  ;[1 1 1] Move Left with Button
  (CallFunction|MoveRightGui -1.0))

(event Custom|OnClickedButtonUp
  ;[1 1 1] Move Forward with Button
  (CallFunction|MoveForwardGui 1.0))

(event EventBeginPlay
  ;[1 1 1] Own Game Mode
  (Utilities|FlowControl|Sequence
    (:then_0
      ;[1 1 1] GUI In Execution Events
      (bind _returnvalue (UserInterface|CreateWidget "/Game/GUI/HUD_In_Execution.HUD_In_Execution_C"))
      (UserInterface|Viewport|AddtoViewport _returnvalue 0)
      (Utilities|FlowControl|Sequence
        (:then_0
          ;[1 1 1] Zoom In and Zoom Out With Slider
          (EventDispatchers|AssignOnZoomSliderChanged _returnvalue (delegate Custom|OnZoomSliderChanged)))
        (:then_1
          ;[1 1 1] Move Forward with Button
          (EventDispatchers|AssignOnClickedButtonUp _returnvalue (delegate Custom|OnClickedButtonUp)))
        (:then_2
          ;[1 1 1] Move Backward with Button
          (EventDispatchers|AssignOnClickedButtonDown _returnvalue (delegate Custom|OnClickedButtonDown)))
        (:then_3
          ;[1 1 1] Move Right with Button
          (EventDispatchers|AssignOnClickedButtonRight _returnvalue (delegate Custom|OnClickedButtonRight)))
        (:then_4
          ;[1 1 1] Move Left with Button
          (EventDispatchers|AssignOnClickedButtonLeft _returnvalue (delegate Custom|OnClickedButtonLeft)))
        (:then_5
          ;[1 1 1] Pause Simulation with Button
          (EventDispatchers|AssignOnClickedButtonPause _returnvalue (delegate Custom|OnClickedButtonPause)))
        (:then_6
          ;[1 1 1] Resume Simulation with Button
          (EventDispatchers|AssignOnClickedButtonResume _returnvalue (delegate Custom|OnClickedButtonResume)))
        (:then_7
          ;[1 1 1] Quit Simulation with Button
          (EventDispatchers|AssignOnClickedButtonQuit _returnvalue (delegate Custom|OnClickedButtonQuit)))))
    (:then_1
      (Input|SetInputModeGameandUI (Game|GetPlayerController 0) 0 "DoNotLock" true)
      (Utilities|Time|SetTimerbyFunctionName 0 "BothMousesCheck" 0.01 true)
      (Utilities|Time|SetTimerbyFunctionName 0 "BothMouses" 0.01 true))))

(event Input|AxisEvents|InputAxisLookRight
  (params (AxisValue :type Float%20%28single-precision%29))
  ;[1 1 1] Look Right and Left with Mouse
  (CallFunction|LookRightLeftMouse))

(event Input|AxisEvents|InputAxisMoveRight
  (params (AxisValue :type Float%20%28single-precision%29))
  ;[1 1 1] Move Left and Right with Keyboard
  (CallFunction|MoveRightKeyboard AxisValue))

(event Input|AxisEvents|InputAxisLookUp
  (params (AxisValue :type Float%20%28single-precision%29))
  ;[1 1 1] Look Up and Down with Mouse
  (CallFunction|LookUpDownMouse))

(event Input|AxisEvents|InputAxisMoveForward
  (params (AxisValue :type Float%20%28single-precision%29))
  ;[1 1 1] Move Forward and Backward with Keyboard
  (CallFunction|MoveForwardKeyboard AxisValue))

(event Input|MouseEvents|LeftMouseButton
  (params (Key :type Key%20Structure :default "None"))
  ;[1 1 1] Setup Control Buttons
  (:Pressed
    (Variables|Default|SetLeftMouseButtonPressed true))
  (:Released
    (Variables|Default|SetLeftMouseButtonPressed false)))

(event Input|MouseEvents|RightMouseButton
  (params (Key :type Key%20Structure :default "None"))
  ;[1 1 1] Setup Control Buttons
  (:Pressed
    (Variables|Default|SetRightMouseButtonPressed true))
  (:Released
    (Variables|Default|SetRightMouseButtonPressed false)))

(event Input|MouseEvents|MouseWheelUp
  (params (Key :type Key%20Structure :default "None"))
  ;[1 1 1] Zoom In and Zoom Out with Mouse
  (:Pressed
    (CallFunction|ZoomMouse 2e+01)))

(event Input|MouseEvents|MouseWheelDown
  (params (Key :type Key%20Structure :default "None"))
  ;[1 1 1] Zoom In and Zoom Out with Mouse
  (:Pressed
    (CallFunction|ZoomMouse -2e+01)))

(event Input|MouseEvents|MouseWheelUp
  (params (Key :type Key%20Structure :default "None"))
  ;[1 1 1] Setup Control Buttons
  (:Pressed
    (Variables|Default|SetMouseWheelUpPressed true))
  (:Released
    (Variables|Default|SetMouseWheelUpPressed false)))

(event Input|MouseEvents|MouseWheelDown
  (params (Key :type Key%20Structure :default "None"))
  ;[1 1 1] Setup Control Buttons
  (:Pressed
    (Variables|Default|SetMouseWheelDownPressed true))
  (:Released
    (Variables|Default|SetMouseWheelDownPressed false)))

(event Input|KeyboardEvents|W
  (params (Key :type Key%20Structure :default "None"))
  ;[1 1 1] Setup Control Buttons
  (:Pressed
    (Variables|Default|SetWKeyPressed true))
  (:Released
    (Variables|Default|SetWKeyPressed false)))

(event Input|KeyboardEvents|S
  (params (Key :type Key%20Structure :default "None"))
  ;[1 1 1] Setup Control Buttons
  (:Pressed
    (Variables|Default|SetSKeyPressed true))
  (:Released
    (Variables|Default|SetSKeyPressed false)))

(event Input|KeyboardEvents|Up
  (params (Key :type Key%20Structure :default "None"))
  ;[1 1 1] Setup Control Buttons
  (:Pressed
    (Variables|Default|SetUpKeyPressed true))
  (:Released
    (Variables|Default|SetUpKeyPressed false)))

(event Input|KeyboardEvents|Down
  (params (Key :type Key%20Structure :default "None"))
  ;[1 1 1] Setup Control Buttons
  (:Pressed
    (Variables|Default|SetDownKeyPressed true))
  (:Released
    (Variables|Default|SetDownKeyPressed false)))

(event Input|KeyboardEvents|A
  (params (Key :type Key%20Structure :default "None"))
  ;[1 1 1] Setup Control Buttons
  (:Pressed
    (Variables|Default|SetAKeyPressed true))
  (:Released
    (Variables|Default|SetDownKeyPressed false)))

(event Input|KeyboardEvents|D
  (params (Key :type Key%20Structure :default "None"))
  ;[1 1 1] Setup Control Buttons
  (:Pressed
    (Variables|Default|SetDKeyPressed true))
  (:Released
    (Variables|Default|SetDKeyPressed false)))

(event Input|KeyboardEvents|Left
  (params (Key :type Key%20Structure :default "None"))
  ;[1 1 1] Setup Control Buttons
  (:Pressed
    (Variables|Default|SetLeftKeyPressed true))
  (:Released
    (Variables|Default|SetLeftKeyPressed false)))

(event Input|KeyboardEvents|Right
  (params (Key :type Key%20Structure :default "None"))
  ;[1 1 1] Setup Control Buttons
  (:Pressed
    (Variables|Default|SetRightKeyPressed true))
  (:Released
    (Variables|Default|SetRightKeyPressed false)))

(fn ConstructionScript)

(fn MoveRightKeyboard
  (params (ScaleValue :type Float%20%28single-precision%29))
  (if (not (Variables|Default|GetBothMouseButtonsPressed))
    (if (Math|Boolean|ORBoolean (Variables|Default|GetAKeyPressed) (Variables|Default|GetDKeyPressed) (Variables|Default|GetLeftKeyPressed) (Variables|Default|GetRightKeyPressed))
      (Pawn|Input|AddMovementInput (Math|Vector|GetRightVector (Math|Rotator|MakeRotator 0.0 0.0 (.Yaw (Math|Rotator|BreakRotator (Pawn|GetControlRotation :!class /Script/Engine.Pawn))))) ScaleValue false))))

(fn MoveRightGui
  (params (ScaleValue :type Float%20%28single-precision%29))
  (Pawn|Input|AddMovementInput (Math|Vector|GetRightVector (Math|Rotator|MakeRotator 0.0 0.0 (.Yaw (Math|Rotator|BreakRotator (Pawn|GetControlRotation :!class /Script/Engine.Pawn))))) ScaleValue false))

(fn MoveForwardKeyboard
  (params (ScaleValue :type Float%20%28single-precision%29))
  (if (not (Variables|Default|GetBothMouseButtonsPressed))
    (if (Math|Boolean|ORBoolean (Variables|Default|GetWKeyPressed) (Variables|Default|GetSKeyPressed) (Variables|Default|GetUpKeyPressed) (Variables|Default|GetDownKeyPressed))
      (Pawn|Input|AddMovementInput (Math|Vector|GetForwardVector (Math|Rotator|MakeRotator 0.0 0.0 (.Yaw (Math|Rotator|BreakRotator (Pawn|GetControlRotation :!class /Script/Engine.Pawn))))) ScaleValue false))))

(fn MoveForwardGui
  (params (ScaleValue :type Float%20%28single-precision%29))
  (Pawn|Input|AddMovementInput (Math|Vector|GetForwardVector (Math|Rotator|MakeRotator 0.0 0.0 (.Yaw (Math|Rotator|BreakRotator (Pawn|GetControlRotation :!class /Script/Engine.Pawn))))) ScaleValue false))

(fn ZoomMouse
  (params (Delta :type Float%20%28single-precision%29))
  (bind _springarm (Variables|Default|GetSpringArm))
  (Variables|/Script/Engine.SpringArmComponent|SetTargetArmLength _springarm (- (Variables|/Script/Engine.SpringArmComponent|GetTargetArmLength _springarm) Delta)))

(fn ZoomGui
  (params (ValueSlider :type Float%20%28single-precision%29))
  (Variables|/Script/Engine.SpringArmComponent|SetTargetArmLength (Variables|Default|GetSpringArm) (- (Variables|Default|GetInitialArmLength) (* ValueSlider 2e+01))))

(fn LookUpDownMouse
  (if (not (Variables|Default|GetBothMouseButtonsPressed))
    (if (Variables|Default|GetRightMouseButtonPressed)
      (bind _result (Math|Float|NegateFloat (Class|Actor|GetInputAxisKeyValue))
        (:%20%20
          (Pawn|Input|AddControllerPitchInput _result))))))

(fn LookRightLeftMouse
  (if (not (Variables|Default|GetBothMouseButtonsPressed))
    (if (or (Variables|Default|GetRightMouseButtonPressed) (Variables|Default|GetLeftMouseButtonPressed))
      (Pawn|Input|AddControllerYawInput (Class|Actor|GetInputAxisKeyValue)))))

(fn SetupBothMousesCheck
  (if (and (Variables|Default|GetLeftMouseButtonPressed) (Variables|Default|GetRightMouseButtonPressed))
    (Variables|Default|SetBothMouseButtonsPressed true)
    (else
      (Variables|Default|SetBothMouseButtonsPressed false))))

(fn SetupBothMouses
  (if (Variables|Default|GetBothMouseButtonsPressed)
    (Pawn|Input|AddMovementInput "0, 0,1.000000" (Class|Actor|GetInputAxisKeyValue) false)
    (Pawn|Input|AddMovementInput (Math|Vector|GetRightVector (Pawn|GetControlRotation :!class /Script/Engine.Pawn)) (Class|Actor|GetInputAxisKeyValue) false)))

(fn PauseSimulation
  (Game|SetGamePaused true)
  (Development|PrintString "The simulation is paused"))

(fn UnPauseSimulation
  (Game|SetGamePaused false)
  (Development|PrintString "The simulation is resumed"))

(fn QuitSimulation
  (Game|QuitGame (Game|GetPlayerController 0) "Quit" false)
  (Development|PrintString "Hasta pronto"))