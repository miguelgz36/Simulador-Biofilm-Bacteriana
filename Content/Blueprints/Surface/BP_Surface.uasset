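; Surface actor for a bacteria simulation that spawns a square grid of block actors from a per-cell type matrix.
; Init runs the empty FillBlocks and DrawBorders stubs around DrawSurface, then either pre-simulates or releases bacteria.
; Pre-simulation spawns a grid of substrate balls above each block, counting down deletion notifications to trigger the release.
; Release spawns a BP_Bacteria_Manager bounded to the central half of each surface axis.
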(event EventBeginPlay)

(event Collision|EventActorBeginOverlap
  (params (OtherActor :type Actor%20Object%20Reference)))

(event EventTick
  (params (DeltaSeconds :type Float%20%28single-precision%29)))

(fn ConstructionScript)

(fn DrawSurface
  ;[1 1 1] Spawn a surface of blocks (Width * Length)
  (for _index (range 0 (- (Variables|Surface|GetWidthBlocks) 1))
    (LocalVariables|SetY _index)
    (Utilities|Array|Add (Variables|Surface|GetBlocks) (Utilities|Struct|MakeS_MatrixActors))
    (for _index_2 (range 0 (- (Variables|Surface|GetLengthBlocks) 1))
      (LocalVariables|SetX _index_2)
      (bind _returnvalue (Game|SpawnActorfromClass (.typeblock (Utilities|Array|Get(acopy) (Utilities|Struct|BreakS_MatrixSurface (Utilities|Array|Get(acopy) (Variables|Surface|GetTypeBlocks) (LocalVariables|GetY))) (LocalVariables|GetX))) (Math|Transform|MakeTransform (Math|Vector|MakeVector (+ (* (.width (Utilities|Array|Get(acopy) (Utilities|Struct|BreakS_MatrixSurface (Utilities|Array|Get(acopy) (Variables|Surface|GetTypeBlocks) (LocalVariables|GetY))) (LocalVariables|GetX))) (Math|Conversions|ToFloat(Integer) (LocalVariables|GetX))) (/ (.width (Utilities|Array|Get(acopy) (Utilities|Struct|BreakS_MatrixSurface (Utilities|Array|Get(acopy) (Variables|Surface|GetTypeBlocks) (LocalVariables|GetY))) (LocalVariables|GetX))) 2.0)) (+ (* (.length (Utilities|Array|Get(acopy) (Utilities|Struct|BreakS_MatrixSurface (Utilities|Array|Get(acopy) (Variables|Surface|GetTypeBlocks) (LocalVariables|GetY))) (LocalVariables|GetX))) (Math|Conversions|ToFloat(Integer) (LocalVariables|GetY))) (/ (.length (Utilities|Array|Get(acopy) (Utilities|Struct|BreakS_MatrixSurface (Utilities|Array|Get(acopy) (Variables|Surface|GetTypeBlocks) (LocalVariables|GetY))) (LocalVariables|GetX))) 2.0)) 0.0)) "AdjustIfPossibleButAlwaysSpawn" 0 0))
      (Utilities|Array|Add (Utilities|Struct|BreakS_MatrixActors (Utilities|Array|Get(acopy) (Variables|Surface|GetBlocks) (LocalVariables|GetY))) _returnvalue))))

(fn FillBlocks
  (params (Surface :type S%20Block%20Structure%20%28by%20ref%29)))

(fn RunPreSimulation
  ;[1 1 1] Matrix travel of type of blocks
  (for (_array_element _array_index) (Variables|Surface|GetTypeBlocks)
    (for (_array_element_2 _array_index_2) (Utilities|Struct|BreakS_MatrixSurface _array_element)
      ;[1 1 1] Loop of number of sustrate balls per block N*M
      (for _index (range 1 5)
        (for _index_2 (range 1 5)
          ;[1 1 1] Create the sustrate ball
          (bind _returnvalue (Game|SpawnActorfromClass "/Game/Blueprints/PreSimulation/BP_SustrateBall.BP_SustrateBall_C" (Math|Transform|MakeTransform (Math|Vector|MakeVector (+ (* _index (/ (.Width (Utilities|Struct|BreakS_Block _array_element_2)) 6.0)) (- (.X (Math|Vector|BreakVector (.Location (Math|Transform|BreakTransform (Transformation|GetActorTransform (Utilities|Array|Get(acopy) (Utilities|Struct|BreakS_MatrixActors (Utilities|Array|Get(acopy) (Variables|Surface|GetBlocks) _array_index)) _array_index_2)))))) (/ (.Width (Utilities|Struct|BreakS_Block _array_element_2)) 2.0))) (+ (* _index_2 (/ (.Length (Utilities|Struct|BreakS_Block _array_element_2)) 6.0)) (- (.Y (Math|Vector|BreakVector (.Location (Math|Transform|BreakTransform (Transformation|GetActorTransform (Utilities|Array|Get(acopy) (Utilities|Struct|BreakS_MatrixActors (Utilities|Array|Get(acopy) (Variables|Surface|GetBlocks) _array_index)) _array_index_2)))))) (/ (.Length (Utilities|Struct|BreakS_Block _array_element_2)) 2.0))) 2e+02)) "AlwaysSpawn" self 0))
          (Variables|/Game/Blueprints/PreSimulation/BP_SustrateBall.BP_SustrateBall_C|SetSurface _returnvalue self)
          (Math|Integer|IncrementInt (Variables|PreSimulation|GetSustrateBallsExisting))))))
  (return))

(fn DrawBorders
  (return))

(fn Init
  (params (NumberBlocks :type Integer%20%28by%20ref%29) (TypeOfBacterium :type BP%20Bacterium%20Class%20Reference%20%28by%20ref%29) (Surface :type S%20Block%20Structure%20%28by%20ref%29) (DoPreSimulation :type Boolean%20%28by%20ref%29))
  ;[1 1 1] Call all functions necessary to initialize surface
  (bind _output_get (Variables|Surface|SetLengthBlocks NumberBlocks))
  (Variables|Surface|SetWidthBlocks _output_get)
  (bind _output_get_2 (Variables|Bacterium|SetBacterium TypeOfBacterium))
  (Surface|FillBlocks Surface)
  (Surface|DrawSurface)
  (Surface|DrawBorders)
  (if DoPreSimulation
    (PreSimulation|RunPreSimulation)
    (else
      (Bacteria|InitializeBacteria _output_get_2)))
  (return))

(fn InitializeBacteria
  (params (TypeOfBacterium :type BP%20Bacterium%20Class%20Reference%20%28by%20ref%29))
  ;[1 1 1] Create a BacteriaManager to control bacteria on the surface
  (bind _returnvalue (Game|SpawnActorfromClass "/Game/Blueprints/Bacteria/BP_Bacteria_Manager.BP_Bacteria_Manager_C" (Math|Transform|MakeTransform "0, 0, 0") "AlwaysSpawn" 0 0))
  ;[1 1 1] Initialize the BacteriaManager to start the release of bacteria on the surface
  (bind (_xlowerbound _xupperbound _ylowerbound _yupperbound) (Surface|GetMapBounds))
  (Default|Init _returnvalue _xlowerbound _xupperbound _ylowerbound _yupperbound TypeOfBacterium)
  (return))

(fn NotifyDeletedBall
  (bind _result (Math|Integer|DecrementInt (Variables|PreSimulation|GetSustrateBallsExisting))
    (:%20%20
      (if (<= _result 0)
        (Bacteria|InitializeBacteria (Variables|Bacterium|GetBacterium)))
      (return))))

(fn GetMapBounds
  (bind _width (Variables|Dimensions|GetWidth))
  (bind _length (Variables|Dimensions|GetLength))
  (bind _returnvalue (/ _length 2.0))
  (bind _returnvalue_2 (/ _width 2.0))
  (bind _returnvalue_3 (- _length _returnvalue))
  (bind _returnvalue_4 (- _width _returnvalue_2))
  (bind _returnvalue_5 (/ _returnvalue_3 2.0))
  (bind _returnvalue_6 (/ _returnvalue_4 2.0))
  (return (- _returnvalue _returnvalue_5) (+ _returnvalue _returnvalue_5) (- _returnvalue_2 _returnvalue_6) (+ _returnvalue_2 _returnvalue_6)))