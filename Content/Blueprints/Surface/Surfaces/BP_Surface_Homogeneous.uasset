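; Surface Blueprint for a homogeneous block grid, where every cell uses the same block type and size.
; FillBlocks builds a WidthBlocks by LengthBlocks matrix of block structs copied from the given surface.
; DrawBorders extends the parent by fitting flat box borders on four sides and the top, sized from the first block.
; It then stores the overall width and length and calls SetPositionCamera.
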(event EventBeginPlay)

(event Collision|EventActorBeginOverlap
  (params (OtherActor :type Actor%20Object%20Reference)))

(event EventTick
  (params (DeltaSeconds :type Float%20%28single-precision%29)))

(fn ConstructionScript)

(fn FillBlocks
  (params (Surface :type S%20Block%20Structure%20%28by%20ref%29))
  (bind (_typeblock _width _length _name) (Utilities|Struct|BreakS_Block Surface))
  ;[1 1 1] Fill the matrix of type of blocks with a type of block
  (for _index (range 0 (- (Variables|Default|GetWidthBlocks) 1))
    (Utilities|Array|Add (Variables|Default|GetTypeBlocks) (Utilities|Struct|MakeS_MatrixSurface))
    (for _index_2 (range 0 (- (Variables|Default|GetLengthBlocks) 1))
      (Utilities|Array|Add (Utilities|Struct|BreakS_MatrixSurface (Utilities|Array|Get(acopy) (Variables|Default|GetTypeBlocks) _index)) (Utilities|Struct|MakeS_Block _typeblock _width _length _name))))
  (return))

(fn DrawBorders
  (bind _lengthblocks (Variables|Default|GetLengthBlocks))
  (bind _widthblocks (Variables|Default|GetWidthBlocks))
  (bind _typeblocks (Variables|Default|GetTypeBlocks))
  (bind _returnvalue (Math|Conversions|ToFloat(Integer) _widthblocks))
  (bind _returnvalue_2 (Math|Conversions|ToFloat(Integer) _lengthblocks))
  (bind _output (Utilities|Array|Get(acopy) _typeblocks))
  (bind _content (Utilities|Struct|BreakS_MatrixSurface _output))
  (bind _output_2 (Utilities|Array|Get(acopy) _content))
  (bind (_typeblock _width _length) (Utilities|Struct|BreakS_Block _output_2))
  (bind _returnvalue_3 (* _width _returnvalue))
  (bind _returnvalue_4 (* _length _returnvalue_2))
  (bind _returnvalue_5 (/ _returnvalue_4 2.0))
  (bind _returnvalue_6 (/ _returnvalue_3 2.0))
  (|CallParentFunction)
  ;[1 1 1] Create borderside0
  (Components|Box|SetBoxExtent (Variables|Default|GetBorderSide0) (Math|Vector|MakeVector _returnvalue_6 0.0 5e+02) false)
  (Transformation|SetWorldTransform (Variables|Default|GetBorderSide0) (Math|Transform|MakeTransform (Math|Vector|MakeVector _returnvalue_6 -1.0 5e+02)) false true)
  ;[1 1 1] Create borderside1
  (Components|Box|SetBoxExtent (Variables|Default|GetBorderSide1) (Math|Vector|MakeVector _returnvalue_6 0.0 5e+02) false)
  (Transformation|SetWorldTransform (Variables|Default|GetBorderSide1) (Math|Transform|MakeTransform (Math|Vector|MakeVector _returnvalue_6 (+ _returnvalue_4 1.0) 5e+02)) false true)
  ;[1 1 1] Create border front
  (Components|Box|SetBoxExtent (Variables|Default|GetBorderFront) (Math|Vector|MakeVector 0.0 _returnvalue_5 5e+02) false)
  (Transformation|SetWorldTransform (Variables|Default|GetBorderFront) (Math|Transform|MakeTransform (Math|Vector|MakeVector -1.0 _returnvalue_5 5e+02)) false true)
  ;[1 1 1] Create border rear
  (Components|Box|SetBoxExtent (Variables|Default|GetBorderRear) (Math|Vector|MakeVector 0.0 _returnvalue_5 5e+02) false)
  (Transformation|SetWorldTransform (Variables|Default|GetBorderRear) (Math|Transform|MakeTransform (Math|Vector|MakeVector (+ _returnvalue_3 1.0) _returnvalue_5 5e+02)) false true)
  ;[1 1 1] Create border top
  (Components|Box|SetBoxExtent (Variables|Default|GetBorderTop) (Math|Vector|MakeVector _returnvalue_6 _returnvalue_5 0.0) false)
  (Transformation|SetWorldTransform (Variables|Default|GetBorderTop) (Math|Transform|MakeTransform (Math|Vector|MakeVector _returnvalue_6 _returnvalue_5 1e+03)) false true)
  (Variables|Default|SetWidth _returnvalue_3)
  (Variables|Default|SetLength _returnvalue_4)
  (CallFunction|SetPositionCamera)
  (return))