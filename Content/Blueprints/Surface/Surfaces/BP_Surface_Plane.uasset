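; BP_Surface_Plane is a surface variant that lays out a rectangular plane of identical blocks.
; On BeginPlay it runs FillBlocks before the parent BeginPlay, so the block layout exists before the parent logic runs.
; FillBlocks extends the parent version, building the TypeBlocks matrix from nested Width and Length loops, with every cell set to a uniformly sized BP_Block_SimpleElevation.
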(event EventBeginPlay
  (CallFunction|FillBlocks)
  (|CallParentFunction))

(event Collision|EventActorBeginOverlap
  (params (OtherActor :type Actor%20Object%20Reference))
  (|CallParentFunction OtherActor) ; This node is disabled and will not be called.\nDrag off pins to build functionality.
)

(event EventTick
  (params (DeltaSeconds :type Float%20%28single-precision%29))
  (|CallParentFunction DeltaSeconds) ; This node is disabled and will not be called.\nDrag off pins to build functionality.
)

(fn ConstructionScript)

(fn FillBlocks
  (|CallParentFunction)
  (for _index (range 0 (Variables|Default|GetWidth))
    (Utilities|Array|Add (Variables|Default|GetTypeBlocks) (Utilities|Struct|MakeMatrixSurface))
    (for _index_2 (range 0 (Variables|Default|GetLength))
      (Utilities|Array|Add (Utilities|Struct|BreakMatrixSurface (Utilities|Array|Get(acopy) (Variables|Default|GetTypeBlocks) _index)) (Utilities|Struct|MakeBlock "/Game/Blueprints/Surface/Surfaces/Blocks/BP_Block_SimpleElevation.BP_Block_SimpleElevation_C" 1e+02 1e+02)))))