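; Bacterium actor that absorbs nutrients on a looping timer and divides by spawning a BP_Bacteria when energy-full, stationary and under its fission limit.
; Spawn points come from scene components: two primary locations, then one random pick of six fallbacks.
; A downward trace validates height, slope and occupancy, then aligns the spawn to the surface with randomized yaw.
; Energy resets even when spawning fails; the math-based DoBinaryFission path is never called here.
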(event Custom|ExecuteLifeCycle
  ;[1 1 1] A timer is set every 0.5 s to execute a custom event for the bacterium
  (InteractionWithEnvironment|GetNutrientsfromEnvironment)
  (bind _isbinarypossible (BinaryFission|VerifyConditionstoFission))
  (if (Math|Boolean|Equal(Boolean) _isbinarypossible true)
    (CallFunction|SpawnUsingComponents)
    (BinaryFission|UpdateBinaryFissionAttempts)))

(event EventBeginPlay
  ;[1 1 1] A timer is set every 0.5 s to execute a custom event for the bacterium
  (Utilities|Time|SetTimerbyEvent (delegate Custom|ExecuteLifeCycle) 0.1 true 2.0))

(event Collision|EventActorBeginOverlap
  (params (OtherActor :type Actor%20Object%20Reference)))

(event EventTick
  (params (DeltaSeconds :type Float%20%28single-precision%29)))

(fn ConstructionScript)

(fn VerifyConditionstoFission
  ;[1 1 1] If the current energy level of the bacterium is greater than the maximum energy level established, the number of attempts to do binary fission is less than 3 and the bacterium is not moving, then the bacterium is able to do binary fission. A boolean value is returned indicating if fission can proceed.
  (return (Math|Boolean|ANDBoolean (>= (Variables|InternalState|GetEnergyLevel) (Variables|Constraints|GetMaximumEnergyLevel)) (< (Variables|InternalState|GetBinaryFissionAttempts) (LocalVariables|GetMaxFissionAttempts)) (Math|Vector|Equal(Vector) (Transformation|GetVelocity) "0, 0, 0" 0.0))))

(fn SetAvailableNutrient
  (params (NewAvailableNutrient :type Float%20%28single-precision%29))
  (Variables|Environment|SetAvailableNutrient NewAvailableNutrient)
  (return))

(fn DoBinaryFission
  ;[1 1 1] According to the return of the function SelectBinaryFissionMethod, a method to do the binary fission is selected, either Simple (return equal to 1) or Complex (return equal to 2)
  (bind _returnvalue (Class|BinaryFission|SelectBinaryFissionMethod (Variables|Default|GetBinaryFission) (Transformation|GetActorRotation)))
  (if (== _returnvalue 1)
    (BinaryFission|SimpleBinaryFission)
    (else
      (BinaryFission|ComplexBinaryFission))))

(fn SimpleBinaryFission
  ;[1 1 1] According to the return of function SelectSimpleFissionWay, a way to try the simple fission is selected, either fission on Y axis (with X coordinate constant, which is the option 1) or fission on X axis (with Y coordinate constant, which is the option 2)
  (bind _returnvalue (Class|BinaryFission|SelectSimpleFissionWay (Variables|Default|GetBinaryFission) (Transformation|GetActorRotation)))
  (BinaryFission|DoSimpleBinaryFission _returnvalue))

(fn DoSimpleBinaryFission
  (params (Option :type Integer))
  (bind _returnvalue (Math|Random|RandomBool))
  (bind _output_get (LocalVariables|SetOptionFission Option))
  ;[1 1 1] The function GetCoordinatesFissionOnYAxis is used to get the location to try a the spawn, then the spawn is tried
  (bind _returnvalue_2 (Class|BinaryFission|GetCoordinatesSimpleFission (Variables|Default|GetBinaryFission) (Transformation|GetActorLocation) (Variables|Dimensions|GetLength) _returnvalue _output_get))
  (bind _spawnstatus (BinaryFission|TrySpawn _returnvalue_2))
  ;[1 1 1] If the previous spawn failed, then the location for spawn is again requested (position on the opposite direction of bacterium) and the spawn is tried again
  (if (Math|Boolean|Equal(Boolean) _spawnstatus false)
    (bind _returnvalue_3 (Class|BinaryFission|GetCoordinatesSimpleFission (Variables|Default|GetBinaryFission) (Transformation|GetActorLocation) (Variables|Dimensions|GetLength) (not _returnvalue) (LocalVariables|GetOptionFission)))
    (bind _spawnstatus_2 (BinaryFission|TrySpawn _returnvalue_3))
    ;[1 1 1] If the spawn failed again in the previous attempt, then a fission is tried using the fission area method
    (if (Math|Boolean|Equal(Boolean) _spawnstatus_2 false)
      (BinaryFission|DoFissionArea))))

(fn DoSpawn
  (params (SpawnTransform :type Transform))
  ;[1 1 1] Tries to spawn a new bacterium with the specified transform
  (bind _returnvalue (Game|SpawnActorfromClass "/Game/Blueprints/Bacteria/BP_Bacteria.BP_Bacteria_C" SpawnTransform "DontSpawnIfColliding" self 0))
  ;[1 1 1] A boolean value is returned, indicating if the spawn was made (true) or failed (false)
  (return (Utilities|IsValid _returnvalue)))

(fn DoFissionArea
  ;[1 1 1] The function GetVectorFissionArea returns a vector indicating the position to try a spawn within surrounding area of bacterium, then the spawn is tried. A boolean value is returned indicating if spawn was done.
  (bind _returnvalue (Class|BinaryFission|GetVectorFissionArea (Variables|Default|GetBinaryFission) (Transformation|GetActorLocation) (Variables|Dimensions|GetLength) (Variables|Dimensions|GetWidth)))
  (bind _spawnstatus (BinaryFission|TrySpawn _returnvalue))
  (return _spawnstatus))

(fn ComplexBinaryFission
  (bind _returnvalue (Math|Random|RandomBool))
  ;[1 1 1] The function GetEquationLine is called to get the intercept and slope of equation of the line (on XY plane) that traverses the bacterium through its center. The parameters are obtained by reference.
  (bind (_slope _intercept) (Class|BinaryFission|GetEquationLine (Variables|Default|GetBinaryFission) (Transformation|GetActorLocation) (Transformation|GetActorRotation) (Math|Trig|GetPI)))
  (bind _output_get (LocalVariables|SetIntercept _intercept))
  (bind _output_get_2 (LocalVariables|SetSlope _slope))
  ;[1 1 1] Fission is tried using the first solution of the intersection between the equation of the line and a circumference (explained in ConsumeNutrients.cpp)
  (bind _wasspawndone (BinaryFission|DoComplexFission _output_get _output_get_2 _returnvalue))
  ;[1 1 1] If the previous fission failed, then the another intersection solution is used to try again
  (if (Math|Boolean|Equal(Boolean) _wasspawndone false)
    (bind _wasspawndone_2 (BinaryFission|DoComplexFission (LocalVariables|GetIntercept) (LocalVariables|GetSlope) (not _returnvalue)))
    ;[1 1 1] If the spawn failed again in the previous attempt, then a fission is tried using the fission area method
    (if (Math|Boolean|Equal(Boolean) _wasspawndone_2 false)
      (BinaryFission|DoFissionArea))))

(fn DoComplexFission
  (params (Intercept :type Float%20%28single-precision%29) (Slope :type Float%20%28single-precision%29) (Choice :type Boolean))
  ;[1 1 1] The function GetIntersectionSolution returns the location for a intersection solution required to spawn, then the spawn is tried. A boolean value indicating if spawn was made is returned.
  (bind _returnvalue (Class|BinaryFission|GetIntersectionSolution (Variables|Default|GetBinaryFission) (Transformation|GetActorLocation) Intercept Slope (Variables|Dimensions|GetLength) Choice))
  (bind _spawnstatus (BinaryFission|TrySpawn _returnvalue))
  (return _spawnstatus))

(fn GetNutrientsfromEnvironment
  ;[1 1 1] The bacterium uses available nutrients from the surface using the function GetNutrients, which increments the energy level of the bacterium depending of available nutrients in environment
  (bind _returnvalue (Class|ConsumeNutrients|GetNutrients (Variables|Default|GetConsumeNutrients) (Variables|Environment|GetAvailableNutrient) (Variables|InternalState|GetEnergyLevel) (Variables|Constraints|GetNutrientAbsorptionRate) (Variables|Constraints|GetMaximumEnergyLevel)))
  (bind _output_get (Variables|InternalState|SetEnergyLevel _returnvalue))
  ;[1 1 1] The nutrient absorption rate is updated according to the energy level of the bacterium
  (bind _returnvalue_2 (Class|ConsumeNutrients|UpdateNutrientAbsorptionRate (Variables|Default|GetConsumeNutrients) _output_get))
  (Variables|Constraints|SetNutrientAbsorptionRate _returnvalue_2))

(fn UpdateBinaryFissionAttempts
  ;[1 1 1] The bacterium do binary fission, creating another instance of bacterium (spawn) in a location and rotation defined by the function DoBinaryFission. After the binary fission, the energy level is reset to 0.0, assuming that the mother cell is now one of the two daughter cells. Also, the variable BinaryFissionAttempts increases by 1.
  (Variables|InternalState|SetEnergyLevel 0.0)
  (Variables|InternalState|SetBinaryFissionAttempts (+ (Variables|InternalState|GetBinaryFissionAttempts) 1.0)))

(fn SetRotationZAxis
  (params (SpawnRotation :type Transform))
  (bind (_location _rotation _scale) (Math|Transform|BreakTransform SpawnRotation))
  (bind (_roll _pitch) (Math|Rotator|BreakRotator _rotation))
  ;[1 1 1] The new transform is established and returned.
  (return (Math|Transform|MakeTransform _location (Math|Rotator|MakeRotator _roll _pitch (+ (.Yaw (Math|Rotator|BreakRotator (Transformation|GetActorRotation))) (Math|Random|RandomFloatinRange -35.0 35.0))) _scale)))

(fn TrySpawn
  (params (SpawnVector :type Vector))
  ;[1 1 1] Using the location to do the spawn in the XY plane, the function GetSpawnTransform returns a boolean value indicating if spawn is viable in that location. If the spawn is viable, the transform returned by the same function (transform adjusted to the height and normal surface) is used to set the rotation of new bacterium on Z axis and then try to spawn, finally returning a boolean indicating if spawn was made. If spawn is not viable (e.g. a bacterium already in that XY position), then a false value is returned.
  (bind (_newtransform _newparam) (RaycastToSpawn|AdjustTransformtoSpawn SpawnVector))
  (if (Math|Boolean|Equal(Boolean) _newparam true)
    (bind _newspawnrotation (BinaryFission|SetRotationZAxis _newtransform))
    (bind _spawnstatus (BinaryFission|DoSpawn _newspawnrotation))
    (return _spawnstatus)
    (else
      (return false))))

(fn LaunchRaycast
  (params (SpawnLocation :type Vector))
  (bind (_x _y) (Math|Vector|BreakVector SpawnLocation))
  ;[1 1 1] The raycast is launched
  (bind (_outhit _returnvalue) (Collision|LineTraceByChannel (Math|Vector|MakeVector _x _y 1e+02) (Math|Vector|MakeVector _x _y -1.0) "TraceTypeQuery1" false 0 "None" false (Class|KismetMathLibrary|LinearColorGreen)))
  ;[1 1 1] The location and the normal vector to the hit surface is obtained, as well as the object type that was hit. A boolean value indicating if there was a hit is returned in first place to ensure a spawn on a surface.
  (return _returnvalue (.Location (Collision|BreakHitResult _outhit)) (.Normal (Collision|BreakHitResult _outhit)) (.HitActor (Collision|BreakHitResult _outhit))))

(fn VerifyActorHit
  (params (ActorHit :type Actor%20Object%20Reference))
  ;[1 1 1] If the object that was hit is a bacterium, then a boolean value of false is returned. Otherwise, a true is returned. This value is used after to determine is spawn is viable, to avoid spawn on another bacterium.
  (return (not (== (Utilities|GetClass ActorHit) "/Game/Blueprints/Bacteria/BP_Bacteria.BP_Bacteria_C"))))

(fn VerifyZCoordinateHit
  (params (Z1Coordinate :type Float%20%28single-precision%29) (Z2Coordinate :type Float%20%28single-precision%29))
  ;[1 1 1] The Z coordinates of both mother cell and the expected new bacterium are compared (the Z coordinate of new bacterium is the Z coordinate of the hit). If the absolute value of this difference is greater than 3 times the width of bacterium, then the spawn is not viable and a boolean value of false is returned. Otherwise, a true value is returned. This avoids to spawn a bacterium within the surrounding area but on an unreachable surface (because of the height), i.e., in a border region.
  (return (not (> (Math|Float|Absolute(Float) (- Z1Coordinate Z2Coordinate)) (* (Variables|Dimensions|GetWidth) 3.0)))))

(fn VerifyInclinationHit
  (params (SpawnRotation :type Rotator))
  (bind (_roll _pitch) (Math|Rotator|BreakRotator SpawnRotation))
  (bind _maxinclination (LocalVariables|GetMaxInclination))
  ;[1 1 1] If rotation on X or Y axis is greater than MaxInclination (in degrees), then spawn is not viable because the inclination is not supported and a false value is returned. Otherwise a true value is returned.
  (return (and (< _roll _maxinclination) (< _pitch _maxinclination))))

(fn GenerateSpawnTransform
  (params (InitialXCoordinate :type Float%20%28single-precision%29) (InitialYCoordinate :type Float%20%28single-precision%29) (ZCoordinateHit :type Float%20%28single-precision%29) (AdjustedRotation :type Rotator))
  (return (Math|Transform|MakeTransform (Math|Vector|MakeVector InitialXCoordinate InitialYCoordinate (+ ZCoordinateHit (Variables|Dimensions|GetWidth))) AdjustedRotation)))

(fn AdjustTransformtoSpawn
  (params (SpawnVector :type Vector))
  (bind (_x _y _z) (Math|Vector|BreakVector SpawnVector))
  ;[1 1 1] If the raycast hit, then the location hit, the normal vector to the surface hit and the hit actor of the raycast are used. From the location the Z coordinate is used to compare against the Z coordinate of mother cell in function VerifyCoordinateHit. The normal vector is used to adjust the rotation of the new bacterium using MakeRotFromZ, then the rotation is reviewed to ensure the inclination contraint and after that to spawn. The hit actor is used to ensure the spawn is possible (avoiding spawning on another bacterium). If there was no hit, then a default transform and a false value is returned.
  (bind (_therewashit _locationhit _normalvectorhit _hitactor) (RaycastToSpawn|LaunchRaycast SpawnVector))
  (if (Math|Boolean|Equal(Boolean) _therewashit true)
    ;[1 1 1] If the three conditions required to have a viable spawn are true, the new transform in created using the function GenerateSpawnTransform, which is returned with a boolean variable with value true indicating the spawn is possible. Otherwise, a default transform and false value are returned. The functions to review the conditions are explained inside each one.
    (bind _iszcoordinatecorrect (RaycastToSpawn|VerifyZCoordinateHit _z (.Z (Math|Vector|BreakVector _locationhit))))
    (bind _isinclinationcorrect (RaycastToSpawn|VerifyInclinationHit (Math|Rotator|MakeRotfromZ _normalvectorhit)))
    (bind _isactorhitcorrect (RaycastToSpawn|VerifyActorHit _hitactor))
    (if (Math|Boolean|ANDBoolean _iszcoordinatecorrect _isinclinationcorrect _isactorhitcorrect)
      (bind _newspawntransform (RaycastToSpawn|GenerateSpawnTransform _x _y (.Z (Math|Vector|BreakVector _locationhit)) (Math|Rotator|MakeRotfromZ _normalvectorhit)))
      (return _newspawntransform true)
      (else
        (return (Math|Transform|MakeTransform "0, 0, 0") false)))
    (else
      (return (Math|Transform|MakeTransform "0, 0, 0") false))))

(fn GetLocationfromComponents
  ;[1 1 1] Get the location of Scene component 1 and set the Location1
  (bind _output_get (LocalVariables|SetLocation1 (Transformation|GetWorldLocation (Variables|Default|GetSpawnSceneComponent1))))
  ;[1 1 1] Get the location of Scene component 2 and set the Location2
  (return _output_get (Transformation|GetWorldLocation (Variables|Default|GetSpawnSceneComponent2))))

(fn SpawnUsingComponents
  ;[1 1 1] Get the location of both Scene components and try to spawn using the location of the first one
  (bind (_firstlocation _secondlocation) (CallFunction|GetLocationfromComponents))
  (bind _spawnstatus (BinaryFission|TrySpawn _firstlocation))
  ;[1 1 1] If the first spawn fails, the second location is used to try again.
  (if (Math|Boolean|Equal(Boolean) _spawnstatus false)
    (bind _spawnstatus_2 (BinaryFission|TrySpawn _secondlocation))
    ;[1 1 1] If the previous spawn fails, then the fission area method is used as last resource
    (if (Math|Boolean|Equal(Boolean) _spawnstatus_2 false)
      (bind _locationcomponent (CallFunction|NewFissionArea))
      (BinaryFission|TrySpawn _locationcomponent))))

(fn NewFissionArea
  (switch int (Math|Random|RandomInteger 6)
    (:0
      (LocalVariables|SetLocationSpawn (Transformation|GetWorldLocation (Variables|Default|GetSpawnSceneComponent3))))
    (:1
      (LocalVariables|SetLocationSpawn (Transformation|GetWorldLocation (Variables|Default|GetSpawnSceneComponent4))))
    (:2
      (LocalVariables|SetLocationSpawn (Transformation|GetWorldLocation (Variables|Default|GetSpawnSceneComponent5))))
    (:3
      (LocalVariables|SetLocationSpawn (Transformation|GetWorldLocation (Variables|Default|GetSpawnSceneComponent6))))
    (:4
      (LocalVariables|SetLocationSpawn (Transformation|GetWorldLocation (Variables|Default|GetSpawnSceneComponent7))))
    (:5
      (LocalVariables|SetLocationSpawn (Transformation|GetWorldLocation (Variables|Default|GetSpawnSceneComponent8)))))
  (return (LocalVariables|GetLocationSpawn)))