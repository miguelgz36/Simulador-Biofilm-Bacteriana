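; Manager actor for a bacterial biofilm simulation that holds shared, temperature-scaled bacteria parameters and controls spawning and death.
; Init pre-spawns a hidden pool through a recursive event that delays every 100 spawns so progress UI can update.
; Colonization drops bacteria at random map locations; later spawns reuse pooled actors, and killed ones return to the pool.
; Each unpaused tick records population and biofilm area, sampling positions every 50 ticks.
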(event Custom|CreateBacteriaCache
  (params (NumberBacteriaCreated :type Integer) (NumberTotalPool :type Integer%20%28by%20ref%29) (Surface :type BP%20Surface%20Object%20Reference))
  ;[1 1 1] Recursive function to recreate a for cycle to spawn bacteria in cache
  (if (< NumberBacteriaCreated NumberTotalPool)
    ;;[1 1 1] For every 100 bacteria created, a delay is made to let UI update of progress
    (if (== (Math|Integer|%(Integer) NumberBacteriaCreated 100) 0)
      (Utilities|FlowControl|Delay 1e-06))
    (InitializeMap|SpawnBacteriumCache)
    (bind _result (Math|Integer|IncrementInt NumberBacteriaCreated)
      (:%20%20
        (Default|IncrementNumberObjectsSpawned Surface)
        (CallFunction|CreateBacteriaCache _result NumberTotalPool Surface)))))

(event EventBeginPlay)

(event Collision|EventActorBeginOverlap
  (params (OtherActor :type Actor%20Object%20Reference)))

(event EventTick
  (params (DeltaSeconds :type Float%20%28single-precision%29))
  (if (not (Variables|Bacteria|GetPaused))
    (Math|Integer|IncrementInt (Variables|Report|GetTickCounter)
      (:%20%20
        (Report|UpdateBacteriaAreaPerTick)))))

(fn ConstructionScript)

(fn DoSpawn
  (params (SpawnTransform :type Transform%20%28by%20ref%29))
  (bind _bacteriapool (Variables|Bacteria|GetBacteriaPool))
  ;[1 1 1] If there is at least one object in BacteriaPool then the first object on the array is used to simulate the creation of a new bacterium (to avoid computational expense). Otherwise, spawn is done to create the new bacterium.
  (if (> (Utilities|Array|Length (Variables|Bacteria|GetBacteriaPool)) 0)
    ;[1 1 1] The first actor in BacteriaPool is used to simulate the spawn. Transform of the actor is changed, then the visibility is enabled, as well as the collisions. After that, that first object is removed from the pool. Finally, a true boolean value is returned indicating that spawn was sucessful.
    (bind _output_get (LocalVariables|SetNewBacterium (Utilities|Array|Get(acopy) _bacteriapool)))
    (Utilities|Array|RemoveIndex _bacteriapool)
    (Transformation|SetActorTransform _output_get SpawnTransform true)
    (Report|AddActiveBacterium (LocalVariables|GetNewBacterium))
    (ManageBacteria|ActivateBacterium (LocalVariables|GetNewBacterium))
    (else
      ;[1 1 1] Try to spawn the new bacterium with the specified transform. If spawn is sucessful, the reference to BacteriaPool is passed to the new bacterium to enable binary fission and a true boolean value is returned. Otherwise, a false value is returned.
      ;;[1 1 1] Tries to spawn a new bacterium with the specified transform
      (bind _returnvalue (Game|SpawnActorfromClass (Variables|Bacteria|GetClassBacteria) SpawnTransform "DontSpawnIfColliding" 0 0))
      ;;[1 1 1] If the spawn was sucessful, the reference to BacteriaPool is passed to the new bacterium. After that, a true boolean value is returned. Otherwise, false is returned.
      (if (Utilities|IsValid _returnvalue)
        (Report|AddActiveBacterium _returnvalue)
        (ManageBacteria|SetInitialInternalStateBacterium _returnvalue)
        (Actor|Tick|SetActorTickEnabled _returnvalue true)
        (else
          (return false)))))
  (return true))

(fn InitializeBacteriaMap
  ;[1 1 1] For the initial number of bacteria established, spawning is done
  (for _index (range 1 (Variables|Bacteria|GetInitialNumberBacteria))
    (InitializeMap|SpawnInitialBacteria)))

(fn SpawnInitialBacteria
  ;[1 1 1] Generate a random transform to spawn the bacterium
  (bind _randomlocation (InitializeMap|GetRandomLocation))
  (bind _randomrotation (InitializeMap|GetRandomRotation))
  ;[1 1 1] Spawn bacterium and show a line raycast in that location
  (bind _returnvalue (Game|SpawnActorfromClass (Variables|Bacteria|GetClassBacteria) (Math|Transform|MakeTransform _randomlocation _randomrotation) "AdjustIfPossibleButAlwaysSpawn" 0 0))
  (InitializeMap|LaunchLineRaycast _randomlocation)
  (Report|AddActiveBacterium _returnvalue)
  ;[1 1 1] Bacterium is able to start on the map
  (ManageBacteria|SetInitialInternalStateBacterium _returnvalue)
  (ManageBacteria|EnablePhysicsBacterium _returnvalue)
  (Default|InitializeColonizingBacterium _returnvalue))

(fn InitializeObjectsPool
  (params (InitialNumberObjectsPool :type Integer%20%28by%20ref%29) (NumberObjectsSpawned :type Integer%20%28by%20ref%29))
  ;[1 1 1] Spawn a initial number of bacteria previous to execution on unused location and without collisions.
  (for _index (range 0 InitialNumberObjectsPool)
    (bind _returnvalue (Game|SpawnActorfromClass (Variables|Bacteria|GetClassBacteria) (Math|Transform|MakeTransform "0, 0, 0") "AlwaysSpawn" 0 0))
    ;[1 1 1] Each new bacterium is hidden from map, its collisions are disabled
    (ManageBacteria|DeactivateBacterium _returnvalue)
    ;[1 1 1] Each bacterium is added to the BacteriaPool
    (Utilities|Array|Add (Variables|Bacteria|GetBacteriaPool) _returnvalue)
    (Math|Integer|IncrementInt NumberObjectsSpawned)))

(fn SetMapBounds
  (params (MapBounds :type S%20Map%20Bounds%20Structure%20%28by%20ref%29))
  (bind (_xlowerbound _xupperbound _ylowerbound _yupperbound) (Utilities|Struct|BreakS_MapBounds MapBounds))
  (Variables|MapBounds|SetXLowerBoundMap _xlowerbound)
  (Variables|MapBounds|SetXUpperBoundMap _xupperbound)
  (Variables|MapBounds|SetYLowerBoundMap _ylowerbound)
  (Variables|MapBounds|SetYUpperBoundMap _yupperbound))

(fn SetInitialNumberBacteria
  (params (InitialNumberBacteria :type Integer))
  (Variables|Bacteria|SetInitialNumberBacteria InitialNumberBacteria))

(fn GetRandomRotation
  (return (Math|Rotator|MakeRotator 0.0 0.0 (Math|Random|RandomFloatinRange 0.0 1.8e+02))))

(fn GetRandomLocation
  (return (Math|Vector|MakeVector (Math|Random|RandomFloatinRange (Variables|MapBounds|GetXLowerBoundMap) (Variables|MapBounds|GetXUpperBoundMap)) (Math|Random|RandomFloatinRange (Variables|MapBounds|GetYLowerBoundMap) (Variables|MapBounds|GetYUpperBoundMap)) (LocalVariables|GetInitialZCoordinate))))

(fn LaunchLineRaycast
  (params (RandomLocation :type Vector%20%28by%20ref%29))
  (bind (_x _y) (Math|Vector|BreakVector RandomLocation))
  (bind _color (LocalVariables|GetColor))
  ;[1 1 1] Generate a line raycast in the spawning location of bacterium during some seconds
  (Collision|LineTraceByChannel (Math|Vector|MakeVector _x _y (LocalVariables|GetMaxZRaycast)) (Math|Vector|MakeVector _x _y (LocalVariables|GetMinZRaycast)) "TraceTypeQuery1" false 0 "ForDuration" true _color _color (LocalVariables|GetDrawTime))
  (return))

(fn AddBacteriumtoPool
  (params (BacteriumReference :type BP%20Bacterium%20Object%20Reference))
  (Utilities|Array|Add (Variables|Bacteria|GetBacteriaPool) BacteriumReference))

(fn Init
  (params (MapBounds :type S%20Map%20Bounds%20Structure%20%28by%20ref%29) (Options :type S%20Options%20Structure%20%28by%20ref%29) (Surface :type BP%20Surface%20Object%20Reference))
  (bind (_bacteria _surface _factornutrientupdatepersize _dopresimulation _presimulationgranularity _blocksperside _temperature _initialenergylevel _maximumenergylevel _nutrientlevelthresholdtomove _minimumenergylevel _energyspenttomove _maximummovementattempts _minimumnutrientlevel _unitsradiustomove _initialnumberbacteriainmemory) (Utilities|Struct|BreakS_Options Options))
  (Setters|SetMapBounds MapBounds)
  (Setters|SetFactorTemperature _temperature)
  (Setters|SetVariablesBacteria _bacteria (* (Variables|Bacteria|GetFactorTemperature) _factornutrientupdatepersize) _initialenergylevel _maximumenergylevel _nutrientlevelthresholdtomove _minimumenergylevel _energyspenttomove _maximummovementattempts _minimumnutrientlevel (* (Variables|Bacteria|GetFactorTemperature) _unitsradiustomove))
  (CallFunction|CreateBacteriaCache 0 _initialnumberbacteriainmemory Surface))

(fn SetInitialInternalStateBacterium
  (params (Bacterium :type BP%20Bacterium%20Object%20Reference))
  (Default|Init Bacterium self (Variables|Bacteria|GetInitialEnergyLevel) (Variables|Bacteria|GetLengthBacterium) (Variables|Bacteria|GetWidthBacterium)))

(fn ActivateBacterium
  (params (Bacterium :type BP%20Bacterium%20Object%20Reference))
  ;[1 1 1] Show actor in the screen, activate collisions and enable tick
  (Rendering|SetActorHiddenInGame Bacterium false)
  (Collision|SetActorEnableCollision Bacterium true)
  (ManageBacteria|SetInitialInternalStateBacterium Bacterium)
  (Actor|Tick|SetActorTickEnabled Bacterium true))

(fn DeactivateBacterium
  (params (Bacterium :type BP%20Bacterium%20Object%20Reference))
  ;[1 1 1] Hide actor in the screen, deactivate collisions and disable tick
  (Actor|Tick|SetActorTickEnabled Bacterium)
  (Rendering|SetActorHiddenInGame Bacterium true)
  (Collision|SetActorEnableCollision Bacterium false))

(fn EnablePhysicsBacterium
  (params (Bacterium :type BP%20Bacterium%20Object%20Reference))
  (bind _staticmesh (Variables|/Game/Blueprints/Bacteria/BP_Bacterium.BP_Bacterium_C|GetStaticMesh Bacterium))
  (Physics|SetEnableGravity _staticmesh true)
  (Physics|SetSimulatePhysics _staticmesh true))

(fn DisablePhysicsBacterium
  (params (Bacterium :type BP%20Bacterium%20Object%20Reference))
  (bind _staticmesh (Variables|/Game/Blueprints/Bacteria/BP_Bacterium.BP_Bacterium_C|GetStaticMesh Bacterium))
  (Physics|SetSimulatePhysics _staticmesh false)
  (Physics|SetEnableGravity _staticmesh false))

(fn EnableFissionInitialBacterium
  (params (Bacterium :type BP%20Bacterium%20Object%20Reference))
  (ManageBacteria|DisablePhysicsBacterium Bacterium)
  (Actor|Tick|SetActorTickEnabled Bacterium true))

(fn AddActiveBacterium
  (params (Bacterium :type BP%20Bacterium%20Object%20Reference))
  (Math|Integer|IncrementInt (Variables|Report|GetBacteriaCounter)
    (:%20%20
      (Utilities|Set|Add (Variables|Bacteria|GetActiveBacteria) Bacterium))))

(fn SubtractActiveBacterium
  (params (Bacterium :type BP%20Bacterium%20Object%20Reference))
  (Math|Integer|DecrementInt (Variables|Report|GetBacteriaCounter)
    (:%20%20
      (Utilities|Set|Remove (Variables|Bacteria|GetActiveBacteria) Bacterium))))

(fn KillBacterium
  (params (Bacterium :type BP%20Bacterium%20Object%20Reference))
  (ManageBacteria|DeactivateBacterium Bacterium)
  (ManageBacteria|AddBacteriumtoPool Bacterium)
  (Report|SubtractActiveBacterium Bacterium))

(fn SetVariablesBacteria
  (params (Bacteria :type S%20Bacterium%20Structure) (FactorNutrientUptakePerSize :type Float%20%28single-precision%29) (InitialEnergyLevel :type Float%20%28single-precision%29) (MaximumEnergyLevel :type Float%20%28single-precision%29) (NutrientLevelThresholdToMove :type Float%20%28single-precision%29) (MinimumEnergyLevel :type Float%20%28single-precision%29) (EnergySpentToMove :type Float%20%28single-precision%29) (MaximumMovementAttempts :type Integer) (MinimumNutrientLevel :type Float%20%28single-precision%29) (UnitsRadiusToMove :type Float%20%28single-precision%29))
  (bind (_name _typebacteria _length _width) (Utilities|Struct|BreakS_Bacterium Bacteria))
  (Variables|Bacteria|SetClassBacteria _typebacteria)
  (bind _output_get (Variables|Bacteria|SetLengthBacterium _length))
  (bind _output_get_2 (Variables|Bacteria|SetWidthBacterium _width))
  (Variables|Bacteria|SetAreaBacterium (* _output_get _output_get_2))
  (Variables|Bacteria|SetFactorNutrientUptakePerSize FactorNutrientUptakePerSize)
  (Variables|Bacteria|SetInitialEnergyLevel InitialEnergyLevel)
  (Variables|Bacteria|SetMaximumEnergyLevel MaximumEnergyLevel)
  (Variables|Bacteria|SetNutrientLevelThresholdToMove NutrientLevelThresholdToMove)
  (Variables|Bacteria|SetMinimumEnergyLevel MinimumEnergyLevel)
  (Variables|Bacteria|SetEnergySpentToMove EnergySpentToMove)
  (Variables|Bacteria|SetMaximumMovementAttempts MaximumMovementAttempts)
  (Variables|Bacteria|SetMinimumNutrientLevel MinimumNutrientLevel)
  (Variables|Bacteria|SetUnitsRadiusToMove UnitsRadiusToMove))

(fn UpdateBacteriaAreaPerTick
  (bind _bacteriacounter (Variables|Report|GetBacteriaCounter))
  (bind _bacteriacounter_2 (Variables|Report|GetBacteriaCounter))
  (Utilities|Array|Add (Variables|Report|GetDataPerTime) (Utilities|Struct|MakeS_SimulationDataPerTime (Variables|Report|GetTickCounter) _bacteriacounter (* _bacteriacounter (Variables|Bacteria|GetAreaBacterium))))
  (if (> (Variables|Report|GetBacteriaCounter) (Variables|Report|GetMaxBacteriaCounter))
    (Variables|Report|SetMaxBacteriaCounter _bacteriacounter_2)
    (Variables|Report|SetMaxBiofilmArea (* _bacteriacounter_2 (Variables|Bacteria|GetAreaBacterium))))
  (if (== (Math|Integer|%(Integer) (Variables|Report|GetTickCounter) 50) 0)
    (bind _result (Utilities|Set|ToArray (Variables|Bacteria|GetActiveBacteria)))
    (for _array_element _result
      (Utilities|Array|Add (Variables|Report|GetBacteriaPositionsPerTime) (Utilities|Struct|MakeS_BacteriaPositionPerTime (Variables|Report|GetTickCounter) (Transformation|GetActorLocation _array_element))))))

(fn GetMaximumEnergyLevel
  (return (Variables|Bacteria|GetMaximumEnergyLevel)))

(fn GetNutrientLevelThresholdtoMove
  (return (Variables|Bacteria|GetNutrientLevelThresholdToMove)))

(fn GetMinimumEnergyLevel
  (return (Variables|Bacteria|GetMinimumEnergyLevel)))

(fn GetEnergySpenttoMove
  (return (Variables|Bacteria|GetEnergySpentToMove)))

(fn GetFactorNutrientUptakePerSize
  (return (Variables|Bacteria|GetFactorNutrientUptakePerSize)))

(fn GetFactorTemperature
  (return (Variables|Bacteria|GetFactorTemperature)))

(fn SetFactorTemperature
  (params (TemperatureEnvironment :type Float%20%28single-precision%29))
  (bind _returnvalue (Class|EstablishFactorTemperature|ComputeFactorTemperature (Variables|Default|GetEstablishFactorTemperature) TemperatureEnvironment))
  (Variables|Bacteria|SetFactorTemperature _returnvalue))

(fn GetMinimumNutrientLevel
  (return (Variables|Bacteria|GetMinimumNutrientLevel)))

(fn GetMaximumMovementAttempts
  (return (Variables|Bacteria|GetMaximumMovementAttempts)))

(fn AdjustTransformInitialBacteria
  (params (Location :type Vector) (Normal :type Vector))
  (bind (_x _y _z) (Math|Vector|BreakVector Location))
  (bind _widthbacterium (Variables|Bacteria|GetWidthBacterium))
  (return (Math|Transform|MakeTransform (Math|Vector|MakeVector _x _y (+ _z (+ _widthbacterium (* _widthbacterium 0.1)))) (Math|Rotator|MakeRotfromZ Normal))))

(fn GetUnitsRadiustoMove
  (return (Variables|Bacteria|GetUnitsRadiusToMove)))

(fn GetBacteriaPositionsonSurface
  (bind _bacteriapositionsonsurface (LocalVariables|GetBacteriaPositionsOnSurface))
  (bind _result (Utilities|Set|ToArray (Variables|Bacteria|GetActiveBacteria)))
  (for _array_element _result
    (Utilities|Array|Add _bacteriapositionsonsurface (Math|Vector2D|MakeVector2D (.X (Math|Vector|BreakVector (Transformation|GetActorLocation _array_element))) (.Y (Math|Vector|BreakVector (Transformation|GetActorLocation _array_element))))))
  (return _bacteriapositionsonsurface))

(fn GetBacteriaDataPerTime
  (return (Variables|Report|GetDataPerTime)))

(fn StartColonization
  (InitializeMap|InitializeBacteriaMap)
  (Actor|Tick|SetActorTickEnabled true))

(fn SpawnBacteriumCache
  ;[1 1 1] Spawn a bacterium previous to execution on unused location and without collisions.
  (bind _returnvalue (Game|SpawnActorfromClass (Variables|Bacteria|GetClassBacteria) (Math|Transform|MakeTransform "0, 0, 0") "AlwaysSpawn" 0 0))
  ;[1 1 1] The bacterium is hidden from map, its collisions are disabled
  (ManageBacteria|DeactivateBacterium _returnvalue)
  ;[1 1 1] The bacterium is added to the BacteriaPool
  (Utilities|Array|Add (Variables|Bacteria|GetBacteriaPool) _returnvalue))

(fn GetMaxBacteriaCounter
  (return (Variables|Report|GetMaxBacteriaCounter)))

(fn GetMaxBiofilmArea
  (return (Variables|Report|GetMaxBiofilmArea)))