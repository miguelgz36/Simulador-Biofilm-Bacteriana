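; Manager actor that scatters an initial population of bacteria across the map at BeginPlay and hands each one the bacteria pool reference.
; Each spawn picks a random XY within map bounds, line-traces down to the surface, then offsets above the hit and aligns to its normal.
; Hits on bacteria or colliding spawns retry through unbounded recursion.
; The random yaw is generated but dropped from the final rotation.
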(event EventBeginPlay
  (InitializeMap|InitializeBacteriaMap))

(event Collision|EventActorBeginOverlap
  (params (OtherActor :type Actor%20Object%20Reference)))

(event EventTick
  (params (DeltaSeconds :type Float%20%28single-precision%29)))

(fn ConstructionScript)

(fn GetRandomTransform
  (params (XLowerBoundMap :type Float%20%28single-precision%29%20%28by%20ref%29) (XUpperBoundMap :type Float%20%28single-precision%29%20%28by%20ref%29) (YLowerBoundMap :type Float%20%28single-precision%29%20%28by%20ref%29) (YUpperBoundMap :type Float%20%28single-precision%29%20%28by%20ref%29))
  (return (Math|Transform|MakeTransform (Math|Vector|MakeVector (Math|Random|RandomFloatinRange XLowerBoundMap XUpperBoundMap) (Math|Random|RandomFloatinRange YLowerBoundMap YUpperBoundMap) 0.0) (Math|Rotator|MakeRotator 0.0 0.0 (Math|Random|RandomFloatinRange (LocalVariables|GetMinRandomRotation) (LocalVariables|GetMaxRandomRotation))))))

(fn LaunchRaycast
  (params (SpawnTransform :type Transform%20%28by%20ref%29))
  (bind _location (Math|Transform|BreakTransform SpawnTransform))
  (bind (_x _y) (Math|Vector|BreakVector _location))
  ;[1 1 1] Launch raycast for the specified XY position. The Z coordinate for start and end are defined by the variables MaxZCoordinate and MinZCoordinate, respectively.
  (bind _outhit (Collision|LineTraceByChannel (Math|Vector|MakeVector _x _y (LocalVariables|GetMaxZCoordinate)) (Math|Vector|MakeVector _x _y (LocalVariables|GetMinZCoordinate)) "TraceTypeQuery1" false 0 "ForDuration" true (LocalVariables|GetColorRaycast) "(R=0.000000,G=1.000000,B=0.000000,A=1.000000)" (LocalVariables|GetDrawTimeRaycast)))
  ;[1 1 1] Return location (of hit) and normal (to surface hit) vectors.
  (return (.Location (Collision|BreakHitResult _outhit)) (.Normal (Collision|BreakHitResult _outhit)) (.HitActor (Collision|BreakHitResult _outhit))))

(fn DoSpawn
  (params (SpawnTransform :type Transform%20%28by%20ref%29))
  ;[1 1 1] Try to spawn a new bacterium in the specified transform
  (bind _returnvalue (Game|SpawnActorfromClass (Variables|Bacteria|GetClassBacteria) SpawnTransform "DontSpawnIfColliding" 0 0))
  ;[1 1 1] If the spawn was sucessful, the reference to BacteriaPool is passed to the new bacterium. After that, a true boolean value is returned. Otherwise, false is returned.
  (if (Utilities|IsValid _returnvalue)
    (Default|SetPoolBacteria _returnvalue (Variables|Bacteria|GetBacteriaPool)))
  (return (Utilities|IsValid _returnvalue)))

(fn SetClassBacteria
  (params (BacteriaType :type BP%20Bacteria%20Class%20Reference%20%28by%20ref%29))
  (Variables|Bacteria|SetClassBacteria BacteriaType))

(fn GetRightRotation
  (params (SpawnTransform :type Transform%20%28by%20ref%29) (LocationHit :type Vector%20%28by%20ref%29) (NormalVectorHit :type Vector%20%28by%20ref%29))
  (bind (_location _rotation) (Math|Transform|BreakTransform SpawnTransform))
  (bind _widthbacteriaobjects (Variables|MapBounds|GetWidthBacteriaObjects))
  (bind (_x _y) (Math|Vector|BreakVector _location))
  (return (Math|Transform|MakeTransform (Math|Vector|MakeVector _x _y (+ (.Z (Math|Vector|BreakVector LocationHit)) (+ _widthbacteriaobjects (* _widthbacteriaobjects 0.1)))) (Math|Rotator|MakeRotfromZ NormalVectorHit))))

(fn InitializeBacteriaMap
  ;[1 1 1] For the initial number of bacteria established, a spawn is done
  (for _index (range 1 (Variables|Bacteria|GetInitialNumberBacteria))
    (InitializeMap|SpawnBacterium)))

(fn SpawnBacterium
  ;[1 1 1] A random location is obtained to try the spawn
  (bind _spawntransform (InitializeMap|GetRandomTransform (Variables|MapBounds|GetXLowerBoundMap) (Variables|MapBounds|GetXUpperBoundMap) (Variables|MapBounds|GetYLowerBoundMap) (Variables|MapBounds|GetYUpperBoundMap)))
  ;[1 1 1] A raycast is launched. If the hit is not on a bacterium, the spawn can be tried. Otherwise, this same function is called again (expecting to get a different random location).
  (bind (_location _normal _hitactor) (InitializeMap|LaunchRaycast _spawntransform))
  (if (!= (Utilities|GetClass _hitactor) (Variables|Bacteria|GetClassBacteria))
    ;[1 1 1] Rotation and Z coordinate are adjusted to the hit surface to try the spawn. If the spawn fails, this function is called again (to get a different random location).
    (bind _newtransform (InitializeMap|GetRightRotation _spawntransform _location _normal))
    (bind _wasspawndone (InitializeMap|DoSpawn _newtransform))
    (if (not _wasspawndone)
      (InitializeMap|SpawnBacterium))
    (else
      (InitializeMap|SpawnBacterium))))