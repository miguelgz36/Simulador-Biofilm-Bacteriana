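; Test bacterium actor that absorbs available nutrients every tick once ready and divides by binary fission when energy is full, attempts remain and it is stationary.
; ConsumeNutrients updates energy and absorption rate; BinaryFission picks simple or complex candidate locations, falling back to a surrounding-area position.
; Line and box traces validate surface, height and free space before BacteriaManager spawns a surface-aligned daughter.
; Otherwise, stationary cells disable physics.
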(event Custom|ExecuteLifeCycle
  ;[1 1 1] A timer is set every 0.5 s to execute a custom event for the bacterium
)

(event EventBeginPlay)

(event Collision|EventActorBeginOverlap
  (params (OtherActor :type Actor%20Object%20Reference)))

(event EventTick
  (params (DeltaSeconds :type Float%20%28single-precision%29))
  (if (Variables|InternalState|GetIsReady)
    (InteractionWithEnvironment|GetNutrientsfromEnvironment)
    (BinaryFission|TryFission)))

(fn ConstructionScript)

(fn VerifyConditionstoFission
  ;[1 1 1] If the current energy level of the bacterium is greater than the maximum energy level established, the number of attempts to do binary fission is less than 3 and the bacterium is not moving, then the bacterium is able to do binary fission. A boolean value is returned indicating if fission can proceed.
  (return (Math|Boolean|ANDBoolean (>= (Variables|InternalState|GetEnergyLevel) (Variables|Constraints|GetMaximumEnergyLevel)) (< (Variables|InternalState|GetBinaryFissionAttempts) (LocalVariables|GetMaxFissionAttempts)) (Math|Vector|Equal(Vector) (Transformation|GetVelocity) "0, 0, 0" 0.0))))

(fn SetAvailableNutrient
  (params (NewAvailableNutrient :type Float%20%28single-precision%29))
  (Variables|Environment|SetAvailableNutrient NewAvailableNutrient)
  (return))

(fn DoBinaryFission
  ;[1 1 1] According to the return of the function SelectBinaryFissionMethod, a method to do the binary fission is selected, either Simple (return equal to 1) or Complex (return equal to 2)
  (bind _returnvalue (Class|BinaryFission|SelectBinaryFissionMethod (Variables|Default|GetBinaryFission) (Transformation|GetActorRotation)))
  (if (== _returnvalue 1)
    (BinaryFission|SimpleBinaryFission)
    (else
      (BinaryFission|ComplexBinaryFission))))

(fn SimpleBinaryFission
  ;[1 1 1] According to the return of function SelectSimpleFissionWay, a way to try the simple fission is selected, either fission on Y axis (with X coordinate constant, which is the option 1) or fission on X axis (with Y coordinate constant, which is the option 2)
  (bind _returnvalue (Class|BinaryFission|SelectSimpleFissionWay (Variables|Default|GetBinaryFission) (Transformation|GetActorRotation)))
  (BinaryFission|DoSimpleBinaryFission _returnvalue))

(fn DoSimpleBinaryFission
  (params (Option :type Integer%20%28by%20ref%29))
  (bind _returnvalue (Math|Random|RandomBool))
  (bind _length (Variables|Dimensions|GetLength))
  (bind _returnvalue_2 (* _length 0.2))
  (bind _returnvalue_3 (+ _length _returnvalue_2))
  (bind _output_get (LocalVariables|SetOptionFission Option))
  ;[1 1 1] The function GetCoordinatesFissionOnYAxis is used to get the location to try spawning, then the spawning is tried
  (bind _returnvalue_4 (Class|BinaryFission|GetCoordinatesSimpleFission (Variables|Default|GetBinaryFission) (Transformation|GetActorLocation) _returnvalue_3 _returnvalue _output_get))
  (bind _spawnstatus (BinaryFission|TrytoSpawn _returnvalue_4))
  ;[1 1 1] If the previous spawn failed, then the location for spawning is again requested (position on the opposite direction of bacterium) and the spawning is tried again
  (if (Math|Boolean|Equal(Boolean) _spawnstatus false)
    (bind _returnvalue_5 (Class|BinaryFission|GetCoordinatesSimpleFission (Variables|Default|GetBinaryFission) (Transformation|GetActorLocation) _returnvalue_3 (not _returnvalue) (LocalVariables|GetOptionFission)))
    (bind _spawnstatus_2 (BinaryFission|TrytoSpawn _returnvalue_5))
    ;[1 1 1] If the spawning failed again in the previous attempt, then a fission is tried using the fission area method
    (if (Math|Boolean|Equal(Boolean) _spawnstatus_2 false)
      (BinaryFission|DoFissionArea))))

(fn DoFissionArea
  (bind _length (Variables|Dimensions|GetLength))
  (bind _width (Variables|Dimensions|GetWidth))
  ;[1 1 1] The function GetVectorFissionArea returns a vector indicating the position to try spawning within surrounding area of bacterium, then the spawn is tried. A boolean value is returned indicating if spawning was done.
  (bind _returnvalue (Class|BinaryFission|GetVectorFissionArea (Variables|Default|GetBinaryFission) (Transformation|GetActorLocation) (+ _length (* _length 0.2)) (+ _width (* _width 0.2))))
  (bind _spawnstatus (BinaryFission|TrytoSpawn _returnvalue))
  (return _spawnstatus))

(fn ComplexBinaryFission
  (bind _returnvalue (Math|Random|RandomBool))
  ;[1 1 1] The function GetEquationLine is called to get the intercept and slope of equation of the line (on XY plane) that traverses the bacterium through its center. The parameters are obtained by reference.
  (bind (_slope _intercept) (Class|BinaryFission|GetEquationLine (Variables|Default|GetBinaryFission) (Transformation|GetActorLocation) (Transformation|GetActorRotation) (Math|Trig|GetPI)))
  (bind _output_get (LocalVariables|SetIntercept _intercept))
  (bind _output_get_2 (LocalVariables|SetSlope _slope))
  ;[1 1 1] Fission is tried using the first solution of the intersection between the equation of the line and a circumference (explained in ConsumeNutrients.cpp)
  (bind _wasspawndone (BinaryFission|DoComplexFission _output_get _output_get_2 _returnvalue))
  ;[1 1 1] If the previous fission failed, then the another intersection solution is used to try again
  (if (Math|Boolean|Equal(Boolean) _wasspawndone false)
    (bind _wasspawndone_2 (BinaryFission|DoComplexFission (LocalVariables|GetIntercept) (LocalVariables|GetSlope) (not _returnvalue)))
    ;[1 1 1] If the spawning failed again in the previous attempt, then a fission is tried using the fission area method
    (if (Math|Boolean|Equal(Boolean) _wasspawndone_2 false)
      (BinaryFission|DoFissionArea))))

(fn DoComplexFission
  (params (Intercept :type Float%20%28single-precision%29%20%28by%20ref%29) (Slope :type Float%20%28single-precision%29%20%28by%20ref%29) (Choice :type Boolean%20%28by%20ref%29))
  (bind _length (Variables|Dimensions|GetLength))
  ;[1 1 1] The function GetIntersectionSolution returns the location for a intersection solution required to spawn, then spawning is tried. A boolean value indicating if spawning was made is returned.
  (bind _returnvalue (Class|BinaryFission|GetIntersectionSolution (Variables|Default|GetBinaryFission) (Transformation|GetActorLocation) Intercept Slope (+ _length (* _length 0.2)) Choice))
  (bind _spawnstatus (BinaryFission|TrytoSpawn _returnvalue))
  (return _spawnstatus))

(fn GetNutrientsfromEnvironment
  (if (> (Variables|Environment|GetAvailableNutrient) 0.0)
    ;[1 1 1] The bacterium uses available nutrients from the surface using the function GetNutrients, which increments the energy level of the bacterium depending of available nutrients in environment
    (bind _returnvalue (Class|ConsumeNutrients|GetNutrients (Variables|Default|GetConsumeNutrients) (Variables|Environment|GetAvailableNutrient) (Variables|InternalState|GetEnergyLevel) (Variables|InternalState|GetNutrientAbsorptionRate) (Variables|Constraints|GetMaximumEnergyLevel)))
    (bind _output_get (Variables|InternalState|SetEnergyLevel _returnvalue))
    ;[1 1 1] The nutrient absorption rate is updated according to the energy level of the bacterium
    (bind _returnvalue_2 (Class|ConsumeNutrients|UpdateNutrientAbsorptionRate (Variables|Default|GetConsumeNutrients) _output_get (Variables|Constraints|GetFactorAbsorption)))
    (Variables|InternalState|SetNutrientAbsorptionRate _returnvalue_2)))

(fn UpdateBinaryFissionAttempts
  ;[1 1 1] The bacterium do binary fission, creating another instance of bacterium in a location and rotation defined by the function DoBinaryFission. After the binary fission, the energy level is reset to 0.0, assuming that the mother cell is now one of the two daughter cells. Also, the variable BinaryFissionAttempts increases by 1.
  (Variables|InternalState|SetEnergyLevel 0.0)
  (Variables|InternalState|SetBinaryFissionAttempts (+ (Variables|InternalState|GetBinaryFissionAttempts) 1)))

(fn SetRotationZAxis
  (params (SpawnTransform :type Transform%20%28by%20ref%29))
  (bind (_location _rotation _scale) (Math|Transform|BreakTransform SpawnTransform))
  (bind (_roll _pitch) (Math|Rotator|BreakRotator _rotation))
  ;[1 1 1] The new transform is established and returned.
  (return (Math|Transform|MakeTransform _location (Math|Rotator|MakeRotator _roll _pitch (+ (.Yaw (Math|Rotator|BreakRotator (Transformation|GetActorRotation))) (Math|Random|RandomFloatinRange (LocalVariables|GetMinRandomRotation) (LocalVariables|GetMaxRandomRotation)))) _scale)))

(fn TrytoSpawn
  (params (SpawnVector :type Vector%20%28by%20ref%29))
  (bind (_therewashit _locationhit _normalvectorhit _hitactor) (RaycastToSpawn|LaunchRaycast SpawnVector))
  ;[1 1 1] If all the conditions are met, spawning can be tried
  (bind _isspawnpossible (RaycastToSpawn|VerifyConditionsSpawn SpawnVector _therewashit _locationhit _hitactor))
  (if _isspawnpossible
    ;[1 1 1] The transform, including the exact Z coordinate to spawn, is finally adjusted
    (bind _newtransform (RaycastToSpawn|AdjustTransformtoSpawn SpawnVector _locationhit _normalvectorhit))
    (bind _newspawntransform (BinaryFission|SetRotationZAxis _newtransform))
    ;[1 1 1] Before trying to spawn, space is verified to ensure spawning can be done in the specified transform.
    (bind _isspaceavailable (BinaryFission|VerifySpacetoSpawn _newspawntransform))
    (if _isspaceavailable
      ;[1 1 1] The BacteriaManager is called to do spawning. The result (done or not) is returned as a boolean value.
      (bind _wasspawndone (Default|DoSpawn (Variables|ObjectReferences|GetBacteriaManager) _newspawntransform (Variables|Environment|GetAvailableNutrient)))
      (if _wasspawndone
        (CallFunction|ResetInternalState))
      (return _wasspawndone)
      (else
        (return false)))
    (else
      (return false))))

(fn LaunchRaycast
  (params (SpawnLocation :type Vector%20%28by%20ref%29))
  (bind (_x _y) (Math|Vector|BreakVector SpawnLocation))
  ;[1 1 1] The raycast is launched
  (bind (_outhit _returnvalue) (Collision|LineTraceByChannel (Math|Vector|MakeVector _x _y (LocalVariables|GetMaxZRaycast)) (Math|Vector|MakeVector _x _y (LocalVariables|GetMinZRaycast)) "TraceTypeQuery1" false 0 "None" false (Class|KismetMathLibrary|LinearColorGreen)))
  ;[1 1 1] The location and the normal vector to the hit surface is obtained, as well as the object type that was hit. A boolean value indicating if there was a hit is returned in first place to ensure a spawn on a surface.
  (return _returnvalue (.Location (Collision|BreakHitResult _outhit)) (.Normal (Collision|BreakHitResult _outhit)) (.HitActor (Collision|BreakHitResult _outhit))))

(fn VerifyActorHit
  (params (ActorHit :type Actor%20Object%20Reference%20%28by%20ref%29))
  ;[1 1 1] If the object that was hit is a bacterium, then a boolean value of false is returned. Otherwise, a true is returned. This value is used after to determine if spawning is viable, to avoid spawning on another bacterium.
  (return (!= (Utilities|GetClass ActorHit) (Utilities|GetClass self))))

(fn VerifyZCoordinateHit
  (params (Z1Coordinate :type Float%20%28single-precision%29%20%28by%20ref%29) (Z2Coordinate :type Float%20%28single-precision%29%20%28by%20ref%29))
  ;[1 1 1] If the Z coordinate to spawn is less than the Z coordinate of mother cell, then true is return, meaning than the new bacterium can fall from above. Otherwise, the flux is passed to the next part.
  (if (< Z1Coordinate Z2Coordinate)
    ;[1 1 1] The Z coordinates of both mother cell and the expected new bacterium are compared (the Z coordinate of new bacterium is the Z coordinate of the hit). If the absolute value of this difference is greater than 3 times the width of bacterium, then spawning is not viable and a boolean value of false is returned. Otherwise, a true value is returned. This avoids to spawn a bacterium within the surrounding area but on an unreachable surface (because of the height), i.e., in a border region.
    (return (not (> (Math|Float|Absolute(Float) (- Z1Coordinate Z2Coordinate)) (* (Variables|Dimensions|GetWidth) (LocalVariables|GetMaxTimesWidthToSpawn)))))
    (else
      (return true))))

(fn AdjustTransformtoSpawn
  (params (SpawnVector :type Vector%20%28by%20ref%29) (LocationHit :type Vector%20%28by%20ref%29) (NormalVectorHit :type Vector%20%28by%20ref%29))
  (bind (_x _y) (Math|Vector|BreakVector SpawnVector))
  (bind _width (Variables|Dimensions|GetWidth))
  (return (Math|Transform|MakeTransform (Math|Vector|MakeVector _x _y (+ (.Z (Math|Vector|BreakVector LocationHit)) (+ _width (* _width 0.1)))) (Math|Rotator|MakeRotfromZ NormalVectorHit))))

(fn SetPoolBacteria
  (params (BacteriaPool :type Array%20of%20BP%20Bacterium%20Object%20References))
  ;[1 1 1] Set the variable BacteriaPool using a parameter by reference to ensure the use of unique pool
)

(fn TryFission
  ;[1 1 1] If conditions to try fission are satisfied then a binary fission is tried.
  (bind _isbinarypossible (BinaryFission|VerifyConditionstoFission))
  (if (Math|Boolean|Equal(Boolean) _isbinarypossible true)
    (BinaryFission|DoBinaryFission)
    (BinaryFission|UpdateBinaryFissionAttempts)
    (else
      (CallFunction|DisablePhysics))))

(fn VerifyConditionsSpawn
  (params (SpawnVector :type Vector%20%28by%20ref%29) (ThereWasHit :type Boolean%20%28by%20ref%29) (LocationHit :type Vector%20%28by%20ref%29) (HitActor :type Actor%20Object%20Reference%20%28by%20ref%29))
  ;[1 1 1] If there was no hit, then the raycast is out of the map and spawning is not possible
  (if ThereWasHit
    ;[1 1 1] If the actor hit by the raycast is not a bacterium, spawning can be tried
    (bind _isactorhitcorrect (RaycastToSpawn|VerifyActorHit HitActor))
    (if _isactorhitcorrect
      ;[1 1 1] If the difference between the Z coordinate of mother cell and new possible bacterium are in the correct range, then spawning is possible
      (bind _iszcoordinatecorrect (RaycastToSpawn|VerifyZCoordinateHit (.Z (Math|Vector|BreakVector SpawnVector)) (.Z (Math|Vector|BreakVector LocationHit))))
      (return _iszcoordinatecorrect)
      (else
        (return false)))
    (else
      (return false))))

(fn VerifySpacetoSpawn
  (params (SpawnTransform :type Transform%20%28by%20ref%29))
  (bind (_location _rotation) (Math|Transform|BreakTransform SpawnTransform))
  (bind _width (Variables|Dimensions|GetWidth))
  (bind (_x _y) (Math|Vector|BreakVector _location))
  (bind _returnvalue (/ _width 2.0))
  ;[1 1 1] A raycast with a box form (BoxTrace) is used to know if there another bacterium in the specified transform.
  (bind _outhit (Collision|BoxTraceByChannel (Math|Vector|MakeVector _x _y 5e+01) (Math|Vector|MakeVector _x _y -1.0) (Math|Vector|MakeVector _returnvalue (/ (Variables|Dimensions|GetLength) 2.0) _returnvalue) _rotation "TraceTypeQuery1" false 0 "None" false))
  ;[1 1 1] If the hit actor is a bacterium, the function returns false. Otherwise, the return is true.
  (return (!= (Utilities|GetClass (.HitActor (Collision|BreakHitResult _outhit))) (Utilities|GetClass self))))

(fn SetBacteriaManager
  (params (BacteriaManager :type BP%20Bacteria%20Manager%20Test%20Object%20Reference))
  (Variables|ObjectReferences|SetBacteriaManager BacteriaManager))

(fn SetReadiness
  (params (IsReady :type Boolean))
  (Variables|InternalState|SetEnergyLevel 0.5)
  (Variables|InternalState|SetNutrientAbsorptionRate 0.125)
  (Variables|InternalState|SetIsReady IsReady))

(fn DisablePhysics
  (bind _staticmesh (Variables|Default|GetStaticMesh))
  ;[1 1 1] If the bacterium is not moving, physics can be disabled.
  (if (Math|Vector|Equal(Vector) (Transformation|GetVelocity) "0, 0, 0" 0.0)
    ;[1 1 1] Disable gravity and other physics.
    (Physics|SetEnableGravity _staticmesh false)
    (Physics|SetSimulatePhysics _staticmesh false)))

(fn ResetInternalState
  (Variables|InternalState|SetNutrientAbsorptionRate 0.8)
  (Variables|InternalState|SetEnergyLevel 1.0))