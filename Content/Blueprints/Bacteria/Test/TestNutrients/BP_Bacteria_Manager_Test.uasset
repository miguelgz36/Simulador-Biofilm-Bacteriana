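; Test bacteria manager that, on BeginPlay, spawns four test bacteria at fixed corners, two with low and two with high nutrient.
; DoSpawn reactivates the first pooled bacterium, or spawns one if collision-free and passes it the manager and nutrient.
; Reused bacteria skip the nutrient assignment; AddBacteriumToPool refills the pool.
; Map-bound, random-placement and debug-trace helpers sit unused by Init, and InitializeBacteriaMap has an empty loop.
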(event EventBeginPlay
  (CallFunction|Init 0.0 0.0 0.0 0.0))

(event Collision|EventActorBeginOverlap
  (params (OtherActor :type Actor%20Object%20Reference)))

(event EventTick
  (params (DeltaSeconds :type Float%20%28single-precision%29)))

(fn ConstructionScript)

(fn DoSpawn
  (params (SpawnTransform :type Transform%20%28by%20ref%29) (Nutrient :type Float%20%28single-precision%29))
  (bind _bacteriapool (Variables|Bacteria|GetBacteriaPool))
  ;[1 1 1] If there is at least one object in BacteriaPool then the first object on the array is used to simulate the creation of a new bacterium (to avoid computational expense). Otherwise, spawn is done to create the new bacterium.
  (if (> (Utilities|Array|Length (Variables|Bacteria|GetBacteriaPool)) 0)
    ;[1 1 1] The first actor in BacteriaPool is used to simulate the spawn. Transform of the actor is changed, then the visibility is enabled, as well as the collisions. After that, that first object is removed from the pool. Finally, a true boolean value is returned indicating that spawn was sucessful.
    (bind _output_get (LocalVariables|SetNewBacterium (Utilities|Array|Get(acopy) _bacteriapool)))
    (Utilities|Array|RemoveIndex _bacteriapool)
    (Transformation|SetActorTransform _output_get SpawnTransform false true)
    (Rendering|SetActorHiddenInGame (LocalVariables|GetNewBacterium) false)
    (Collision|SetActorEnableCollision (LocalVariables|GetNewBacterium) true)
    (Default|SetReadiness (LocalVariables|GetNewBacterium) true)
    (return true)
    (else
      ;[1 1 1] Try to spawn the new bacterium with the specified transform. If spawn is sucessful, the reference to BacteriaPool is passed to the new bacterium to enable binary fission and a true boolean value is returned. Otherwise, a false value is returned.
      ;;[1 1 1] Tries to spawn a new bacterium with the specified transform
      (bind _returnvalue (Game|SpawnActorfromClass (Variables|Bacteria|GetClassBacteria) SpawnTransform "DontSpawnIfColliding" 0 0))
      ;;[1 1 1] If the spawn was sucessful, the reference to BacteriaPool is passed to the new bacterium. After that, a true boolean value is returned. Otherwise, false is returned.
      (if (Utilities|IsValid _returnvalue)
        (Default|SetBacteriaManager _returnvalue self)
        (Default|SetAvailableNutrient _returnvalue Nutrient)
        (Default|SetReadiness _returnvalue true))
      (return (Utilities|IsValid _returnvalue)))))

(fn SetClassBacteria
  (params (BacteriaType :type BP%20Bacteria%20Test%20Class%20Reference%20%28by%20ref%29))
  (Variables|Bacteria|SetClassBacteria BacteriaType))

(fn InitializeBacteriaMap
  ;[1 1 1] For the initial number of bacteria established, spawning is done
  (for _index (range 1 (Variables|Bacteria|GetInitialNumberBacteria))
    _))

(fn SetMapBounds
  (params (XLowerBound :type Float%20%28single-precision%29) (XUpperBound :type Float%20%28single-precision%29) (YLowerBound :type Float%20%28single-precision%29) (YUpperBound :type Float%20%28single-precision%29))
  (Variables|MapBounds|SetXLowerBoundMap XLowerBound)
  (Variables|MapBounds|SetXUpperBoundMap XUpperBound)
  (Variables|MapBounds|SetYLowerBoundMap YLowerBound)
  (Variables|MapBounds|SetYUpperBoundMap YUpperBound))

(fn SetInitialNumberBacteria
  (params (InitialNumberBacteria :type Integer))
  (Variables|Bacteria|SetInitialNumberBacteria InitialNumberBacteria))

(fn GetRandomRotation
  (return (Math|Rotator|MakeRotator 0.0 0.0 (Math|Random|RandomFloatinRange 0.0 1.8e+02))))

(fn GetRandomLocation
  (return (Math|Vector|MakeVector (Math|Random|RandomFloatinRange (Variables|MapBounds|GetXLowerBoundMap) (Variables|MapBounds|GetXUpperBoundMap)) (Math|Random|RandomFloatinRange (Variables|MapBounds|GetYLowerBoundMap) (Variables|MapBounds|GetYUpperBoundMap)) (LocalVariables|GetInitialZCoordinate))))

(fn ShowLineRaycast
  (params (RandomLocation :type Vector%20%28by%20ref%29))
  (bind (_x _y) (Math|Vector|BreakVector RandomLocation))
  (bind _color (LocalVariables|GetColor))
  ;[1 1 1] Generate a line raycast in the spawning location of bacterium during some seconds
  (Collision|LineTraceByChannel RandomLocation (Math|Vector|MakeVector _x _y -1.0) "TraceTypeQuery1" false 0 "ForDuration" true _color _color (LocalVariables|GetDrawTime)))

(fn AddBacteriumtoPool
  (params (BacteriumReference :type BP%20Bacterium%20Object%20Reference))
  (Utilities|Array|Add (Variables|Bacteria|GetBacteriaPool) BacteriumReference))

(fn Init
  (params (XLowerBound :type Float%20%28single-precision%29) (XUpperBound :type Float%20%28single-precision%29) (YLowerBound :type Float%20%28single-precision%29) (YUpperBound :type Float%20%28single-precision%29) (BacteriaType :type BP%20Bacterium%20Class%20Reference))
  (Variables|Bacteria|SetClassBacteria "/Game/Blueprints/Bacteria/Test/TestNutrients/BP_Bacteria_Test.BP_Bacteria_Test_C")
  (ManageBacteria|DoSpawn (Math|Transform|MakeTransform "-250.000000,-250.000000,1.700000") 0.1)
  (ManageBacteria|DoSpawn (Math|Transform|MakeTransform "-250.000000,250.000000,1.700000") 0.1)
  (ManageBacteria|DoSpawn (Math|Transform|MakeTransform "250.000000,-250.000000,1.700000") 1.2)
  (ManageBacteria|DoSpawn (Math|Transform|MakeTransform "250.000000,250.000000,1.700000") 1.2))