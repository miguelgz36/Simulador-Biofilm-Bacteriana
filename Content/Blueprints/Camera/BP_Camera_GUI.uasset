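; BP_Camera_GUI provides GUI-facing controls for moving a camera pawn and managing the simulation.
; InitGUI stores the target Pawn, which the move functions drive with scaled movement input: forward and right follow control yaw only, while up uses world Z.
; Separate functions pause, resume or quit the simulation, each printing a status or farewell message.
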(fn MoveRightGui
  (params (Scale :type Float%20%28single-precision%29))
  (Pawn|Input|AddMovementInput (Variables|Default|GetPawn) (Math|Vector|GetRightVector (Math|Rotator|MakeRotator 0.0 0.0 (.Yaw (Math|Rotator|BreakRotator (Pawn|GetControlRotation (Variables|Default|GetPawn) :!class /Script/Engine.Pawn))))) Scale false))

(fn MoveForwardGui
  (params (Scale :type Float%20%28single-precision%29))
  (Pawn|Input|AddMovementInput (Variables|Default|GetPawn) (Math|Vector|GetForwardVector (Math|Rotator|MakeRotator 0.0 0.0 (.Yaw (Math|Rotator|BreakRotator (Pawn|GetControlRotation (Variables|Default|GetPawn) :!class /Script/Engine.Pawn))))) Scale false))

(fn MoveUpGui
  (params (Scale :type Float%20%28single-precision%29))
  (Pawn|Input|AddMovementInput (Variables|Default|GetPawn) "0, 0,1.000000" Scale false))

(fn PauseSimulation
  (Game|SetGamePaused true)
  (Development|PrintString "The simulation is paused"))

(fn ResumeSimulation
  (Game|SetGamePaused false)
  (Development|PrintString "The simulation is resumed"))

(fn QuitSimulation
  (Game|QuitGame (Game|GetPlayerController 0) "Quit" false)
  (Development|PrintString "Hasta pronto"))

(fn InitGUI
  (params (Pawn :type BP%20Pawn%20Object%20Reference))
  (Variables|Default|SetPawn Pawn))