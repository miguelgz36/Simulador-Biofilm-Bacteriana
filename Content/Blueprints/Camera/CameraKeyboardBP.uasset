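; Keyboard and mouse camera control helper that drives a Character reference passed in through InitKeyboard.
; Move functions check the Character's key flags: WASD and left/right arrows add movement along control yaw only, while up/down arrows offset its Scene component vertically.
; Look functions feed controller input only while mouse buttons are held: right for pitch, either right or left for yaw.
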(event EventBeginPlay)

(event EventTick
  (params (DeltaSeconds :type Float%20%28single-precision%29)))

(fn MoveRightKeyboard
  (params (ScaleValue :type Float%20%28single-precision%29))
  (if (Math|Boolean|ORBoolean (Variables|/Game/Blueprints/Camera/CharacterBP.CharacterBP_C|GetAKeyPressed (Variables|Default|GetCharacter)) (Variables|/Game/Blueprints/Camera/CharacterBP.CharacterBP_C|GetDKeyPressed (Variables|Default|GetCharacter)) (Variables|/Game/Blueprints/Camera/CharacterBP.CharacterBP_C|GetRightKeyPressed (Variables|Default|GetCharacter)) (Variables|/Game/Blueprints/Camera/CharacterBP.CharacterBP_C|GetLeftKeyPressed (Variables|Default|GetCharacter)))
    (Pawn|Input|AddMovementInput (Variables|Default|GetCharacter) (Math|Vector|GetRightVector (Math|Rotator|MakeRotator 0.0 0.0 (.Yaw (Math|Rotator|BreakRotator (Pawn|GetControlRotation (Variables|Default|GetCharacter) :!class /Script/Engine.Pawn))))) ScaleValue false)))

(fn MoveForwardKeyboard
  (params (ScaleValue :type Float%20%28single-precision%29))
  (if (or (Variables|/Game/Blueprints/Camera/CharacterBP.CharacterBP_C|GetWKeyPressed (Variables|Default|GetCharacter)) (Variables|/Game/Blueprints/Camera/CharacterBP.CharacterBP_C|GetSKeyPressed (Variables|Default|GetCharacter)))
    (Pawn|Input|AddMovementInput (Variables|Default|GetCharacter) (Math|Vector|GetForwardVector (Math|Rotator|MakeRotator 0.0 0.0 (.Yaw (Math|Rotator|BreakRotator (Pawn|GetControlRotation (Variables|Default|GetCharacter) :!class /Script/Engine.Pawn))))) ScaleValue false)))

(fn MoveUpKeyboard
  (params (ScaleValue :type Float%20%28single-precision%29))
  (if (or (Variables|/Game/Blueprints/Camera/CharacterBP.CharacterBP_C|GetUpKeyPressed (Variables|Default|GetCharacter)) (Variables|/Game/Blueprints/Camera/CharacterBP.CharacterBP_C|GetDownKeyPressed (Variables|Default|GetCharacter)))
    (Transformation|AddLocalOffset (Variables|/Game/Blueprints/Camera/CharacterBP.CharacterBP_C|GetScene (Variables|Default|GetCharacter)) (Math|Vector|MakeVector 0.0 0.0 (* ScaleValue 1e+01)) false false)))

(fn LookUpDownMouse
  (params (MouseY :type Float%20%28single-precision%29))
  (if (Variables|/Game/Blueprints/Camera/CharacterBP.CharacterBP_C|GetRightMouseButtonPressed (Variables|Default|GetCharacter))
    (bind _result (Math|Float|NegateFloat MouseY)
      (:%20%20
        (Pawn|Input|AddControllerPitchInput (Variables|Default|GetCharacter) _result)))))

(fn LookRightLeftMouse
  (params (MouseX :type Float%20%28single-precision%29))
  (if (or (Variables|/Game/Blueprints/Camera/CharacterBP.CharacterBP_C|GetRightMouseButtonPressed (Variables|Default|GetCharacter)) (Variables|/Game/Blueprints/Camera/CharacterBP.CharacterBP_C|GetLeftMouseButtonPressed (Variables|Default|GetCharacter)))
    (Pawn|Input|AddControllerYawInput (Variables|Default|GetCharacter) MouseX)))

(fn InitKeyboard
  (params (Character :type Character%20BP%20Object%20Reference))
  (Variables|Default|SetCharacter Character))