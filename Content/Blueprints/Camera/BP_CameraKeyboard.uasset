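; Camera input helper that turns mouse movement into look rotation for a character.
; InitKeyboard stores the character reference that both look functions act on.
; While that character's left or right mouse button is flagged as pressed, MouseX feeds controller yaw and MouseY, after a conversion step, feeds controller pitch.
; BeginPlay and Tick are unused, so the functions rely on external calls.
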(event EventBeginPlay)

(event EventTick
  (params (DeltaSeconds :type Float%20%28single-precision%29)))

(fn LookUpDownMouse
  (params (MouseY :type Float%20%28single-precision%29))
  (if (or (Variables|/Game/Blueprints/Camera/BP_Character.BP_Character_C|GetRightMouseButtonPressed (Variables|Default|GetCharacter)) (Variables|/Game/Blueprints/Camera/BP_Character.BP_Character_C|GetLeftMouseButtonPressed (Variables|Default|GetCharacter)))
    (bind _result (Math|Float|NegateFloat MouseY)
      (:%20%20
        (Pawn|Input|AddControllerPitchInput (Variables|Default|GetCharacter) _result)))))

(fn LookRightLeftMouse
  (params (MouseX :type Float%20%28single-precision%29))
  (if (or (Variables|/Game/Blueprints/Camera/BP_Character.BP_Character_C|GetRightMouseButtonPressed (Variables|Default|GetCharacter)) (Variables|/Game/Blueprints/Camera/BP_Character.BP_Character_C|GetLeftMouseButtonPressed (Variables|Default|GetCharacter)))
    (Pawn|Input|AddControllerYawInput (Variables|Default|GetCharacter) MouseX)))

(fn InitKeyboard
  (params (Character :type BP%20Character%20Object%20Reference))
  (Variables|Default|SetCharacter Character))