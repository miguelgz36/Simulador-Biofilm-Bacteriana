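; Player character Blueprint that serves as the input hub for a controllable camera.
; On BeginPlay it passes itself to CameraKeyboardBP and CameraInterfaceBP components for initialization.
; Mouse and movement axes forward to CameraKeyboardBP for looking and moving along three axes, while the mouse wheel feeds CameraInterfaceBP's speed factor.
; Mouse button, WASD and arrow key events record held state in boolean flags.
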(event EventBeginPlay
  ;[1 1 1] Init CameraInterfaceBP and CameraKeyboardBP Components
  (Default|InitKeyboard (Variables|Default|GetCameraKeyboardBP) self)
  (Default|InitInterface (Variables|Default|GetCameraInterfaceBP) self))

(event Input|AxisEvents|InputAxisMouseX
  (params (AxisValue :type Float%20%28single-precision%29))
  ;[1 1 1] Look Right and Left with Mouse
  (Default|LookRightLeftMouse (Variables|Default|GetCameraKeyboardBP) AxisValue))

(event Input|AxisEvents|InputAxisMouseY
  (params (AxisValue :type Float%20%28single-precision%29))
  ;[1 1 1] Look Up and Down with Mouse
  (Default|LookUpDownMouse (Variables|Default|GetCameraKeyboardBP) AxisValue))

(event Input|AxisEvents|InputAxisMoveRight
  (params (AxisValue :type Float%20%28single-precision%29))
  ;[1 1 1] Move Left and Right with Keyboard
  (Default|MoveRightKeyboard (Variables|Default|GetCameraKeyboardBP) AxisValue))

(event Input|AxisEvents|InputAxisMoveForward
  (params (AxisValue :type Float%20%28single-precision%29))
  ;[1 1 1] Move Forward and Backward with Keyboard
  (Default|MoveForwardKeyboard (Variables|Default|GetCameraKeyboardBP) AxisValue))

(event Input|AxisEvents|InputAxisMoveUp
  (params (AxisValue :type Float%20%28single-precision%29))
  ;[1 1 1] Move Up and Down with Keyboard
  (Default|MoveUpKeyboard (Variables|Default|GetCameraKeyboardBP) AxisValue))

(event Input|MouseEvents|MouseWheelAxis
  (params (AxisValue :type Float%20%28single-precision%29))
  ;[1 1 1] Increase Velocity of camera
  (bind _result (Math|Float|NegateFloat AxisValue)
    (:%20%20
      (Default|SetFactor (Variables|Default|GetCameraInterfaceBP) _result))))

(event Input|MouseEvents|LeftMouseButton
  (params (Key :type Key%20Structure :default "None"))
  ;[1 1 1] Setup Control Buttons
  (:Pressed
    (Variables|Default|SetLeftMouseButtonPressed true))
  (:Released
    (Variables|Default|SetLeftMouseButtonPressed false)))

(event Input|MouseEvents|RightMouseButton
  (params (Key :type Key%20Structure :default "None"))
  ;[1 1 1] Setup Control Buttons
  (:Pressed
    (Variables|Default|SetRightMouseButtonPressed true))
  (:Released
    (Variables|Default|SetRightMouseButtonPressed false)))

(event Input|KeyboardEvents|W
  (params (Key :type Key%20Structure :default "None"))
  ;[1 1 1] Setup Control Buttons
  (:Pressed
    (Variables|Default|SetWKeyPressed true))
  (:Released
    (Variables|Default|SetWKeyPressed false)))

(event Input|KeyboardEvents|S
  (params (Key :type Key%20Structure :default "None"))
  ;[1 1 1] Setup Control Buttons
  (:Pressed
    (Variables|Default|SetSKeyPressed true))
  (:Released
    (Variables|Default|SetSKeyPressed false)))

(event Input|KeyboardEvents|Up
  (params (Key :type Key%20Structure :default "None"))
  ;[1 1 1] Setup Control Buttons
  (:Pressed
    (Variables|Default|SetUpKeyPressed true))
  (:Released
    (Variables|Default|SetUpKeyPressed false)))

(event Input|KeyboardEvents|Down
  (params (Key :type Key%20Structure :default "None"))
  ;[1 1 1] Setup Control Buttons
  (:Pressed
    (Variables|Default|SetDownKeyPressed true))
  (:Released
    (Variables|Default|SetDownKeyPressed false)))

(event Input|KeyboardEvents|A
  (params (Key :type Key%20Structure :default "None"))
  ;[1 1 1] Setup Control Buttons
  (:Pressed
    (Variables|Default|SetAKeyPressed true))
  (:Released
    (Variables|Default|SetDownKeyPressed false)))

(event Input|KeyboardEvents|D
  (params (Key :type Key%20Structure :default "None"))
  ;[1 1 1] Setup Control Buttons
  (:Pressed
    (Variables|Default|SetDKeyPressed true))
  (:Released
    (Variables|Default|SetDKeyPressed false)))

(event Input|KeyboardEvents|Left
  (params (Key :type Key%20Structure :default "None"))
  ;[1 1 1] Setup Control Buttons
  (:Pressed
    (Variables|Default|SetLeftKeyPressed true))
  (:Released
    (Variables|Default|SetLeftKeyPressed false)))

(event Input|KeyboardEvents|Right
  (params (Key :type Key%20Structure :default "None"))
  ;[1 1 1] Setup Control Buttons
  (:Pressed
    (Variables|Default|SetRightKeyPressed true))
  (:Released
    (Variables|Default|SetRightKeyPressed false)))

(fn ConstructionScript)