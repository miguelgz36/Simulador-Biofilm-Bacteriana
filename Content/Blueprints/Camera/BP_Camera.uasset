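; BP_Camera is a player-controlled camera that moves by keyboard and looks around with the mouse.
; It records mouse button, WASD and arrow key states as booleans, though releasing A clears the Down flag instead of its own.
; Look and move axis events delegate to BPCameraKeyboard.
; Both-mouse-button events delegate there too, but the looping timers meant to poll them are unconnected and never run.
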(event Custom|BothMouses
  ;[1 1 1] Setup Both Mouse Buttons
  (Default|SetupBothMouses (Variables|Default|GetBP_Camera_Keyboard)))

(event Custom|BothMousesCheck
  ;[1 1 1] Setup Both Mouse Buttons
  (Default|SetupBothMousesCheck (Variables|Default|GetBP_Camera_Keyboard)))

(event Input|AxisEvents|InputAxisMoveUp
  (params (AxisValue :type Float%20%28single-precision%29))
  ;[1 1 1] Move Up and Down with Keyboard
  (Default|MoveUpKeyboard (Variables|Default|GetBP_Camera_Keyboard) AxisValue))

(event Input|AxisEvents|InputAxisLookRight
  (params (AxisValue :type Float%20%28single-precision%29))
  ;[1 1 1] Look Right and Left with Mouse
  (Default|LookRightLeftMouse (Variables|Default|GetBP_Camera_Keyboard)))

(event Input|AxisEvents|InputAxisMoveRight
  (params (AxisValue :type Float%20%28single-precision%29))
  ;[1 1 1] Move Left and Right with Keyboard
  (Default|MoveRightKeyboard (Variables|Default|GetBP_Camera_Keyboard) AxisValue))

(event Input|AxisEvents|InputAxisLookUp
  (params (AxisValue :type Float%20%28single-precision%29))
  ;[1 1 1] Look Up and Down with Mouse
  (Default|LookUpDownMouse (Variables|Default|GetBP_Camera_Keyboard)))

(event Input|AxisEvents|InputAxisMoveForward
  (params (AxisValue :type Float%20%28single-precision%29))
  ;[1 1 1] Move Forward and Backward with Keyboard
  (Default|MoveForwardKeyboard (Variables|Default|GetBP_Camera_Keyboard) AxisValue))

(event Input|MouseEvents|LeftMouseButton
  (params (Key :type Key%20Structure :default "None"))
  ;[1 1 1] Setup Control Buttons
  (:Pressed
    (Variables|Default|SetLeftMouseButtonPressed true))
  (:Released
    (Variables|Default|SetLeftMouseButtonPressed false)))

(event Input|MouseEvents|RightMouseButton
  (params (Key :type Key%20Structure :default "None"))
  ;[1 1 1] Setup Control Buttons
  (:Pressed
    (Variables|Default|SetRightMouseButtonPressed true))
  (:Released
    (Variables|Default|SetRightMouseButtonPressed false)))

(event Input|KeyboardEvents|W
  (params (Key :type Key%20Structure :default "None"))
  ;[1 1 1] Setup Control Buttons
  (:Pressed
    (Variables|Default|SetWKeyPressed true))
  (:Released
    (Variables|Default|SetWKeyPressed false)))

(event Input|KeyboardEvents|S
  (params (Key :type Key%20Structure :default "None"))
  ;[1 1 1] Setup Control Buttons
  (:Pressed
    (Variables|Default|SetSKeyPressed true))
  (:Released
    (Variables|Default|SetSKeyPressed false)))

(event Input|KeyboardEvents|Up
  (params (Key :type Key%20Structure :default "None"))
  ;[1 1 1] Setup Control Buttons
  (:Pressed
    (Variables|Default|SetUpKeyPressed true))
  (:Released
    (Variables|Default|SetUpKeyPressed false)))

(event Input|KeyboardEvents|Down
  (params (Key :type Key%20Structure :default "None"))
  ;[1 1 1] Setup Control Buttons
  (:Pressed
    (Variables|Default|SetDownKeyPressed true))
  (:Released
    (Variables|Default|SetDownKeyPressed false)))

(event Input|KeyboardEvents|A
  (params (Key :type Key%20Structure :default "None"))
  ;[1 1 1] Setup Control Buttons
  (:Pressed
    (Variables|Default|SetAKeyPressed true))
  (:Released
    (Variables|Default|SetDownKeyPressed false)))

(event Input|KeyboardEvents|D
  (params (Key :type Key%20Structure :default "None"))
  ;[1 1 1] Setup Control Buttons
  (:Pressed
    (Variables|Default|SetDKeyPressed true))
  (:Released
    (Variables|Default|SetDKeyPressed false)))

(event Input|KeyboardEvents|Left
  (params (Key :type Key%20Structure :default "None"))
  ;[1 1 1] Setup Control Buttons
  (:Pressed
    (Variables|Default|SetLeftKeyPressed true))
  (:Released
    (Variables|Default|SetLeftKeyPressed false)))

(event Input|KeyboardEvents|Right
  (params (Key :type Key%20Structure :default "None"))
  ;[1 1 1] Setup Control Buttons
  (:Pressed
    (Variables|Default|SetRightKeyPressed true))
  (:Released
    (Variables|Default|SetRightKeyPressed false)))

(fn ConstructionScript)