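; Keyboard and mouse control logic for a camera pawn, which InitKeyboard passes in and stores.
; Key flags on the pawn gate yaw-relative horizontal movement and world-Z vertical movement.
; Right mouse drives pitch and either button drives yaw, while holding both suppresses look and horizontal key movement to pan vertically and sideways.
; Look and pan amounts come from the player controller's mouse position.
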(fn MoveRightKeyboard
  (params (Scale :type Float%20%28single-precision%29))
  (if (not (Variables|/Game/Blueprints/Camera/BP_Pawn.BP_Pawn_C|GetBothMouseButtonsPressed (Variables|Default|GetPawn)))
    (if (Math|Boolean|ORBoolean (Variables|/Game/Blueprints/Camera/BP_Pawn.BP_Pawn_C|GetAKeyPressed (Variables|Default|GetPawn)) (Variables|/Game/Blueprints/Camera/BP_Pawn.BP_Pawn_C|GetDKeyPressed (Variables|Default|GetPawn)) (Variables|/Game/Blueprints/Camera/BP_Pawn.BP_Pawn_C|GetLeftKeyPressed (Variables|Default|GetPawn)) (Variables|/Game/Blueprints/Camera/BP_Pawn.BP_Pawn_C|GetRightKeyPressed (Variables|Default|GetPawn)))
      (Pawn|Input|AddMovementInput (Variables|Default|GetPawn) (Math|Vector|GetRightVector (Math|Rotator|MakeRotator 0.0 0.0 (.Yaw (Math|Rotator|BreakRotator (Pawn|GetControlRotation (Variables|Default|GetPawn) :!class /Script/Engine.Pawn))))) Scale false))))

(fn MoveForwardKeyboard
  (params (Scale :type Float%20%28single-precision%29))
  (if (not (Variables|/Game/Blueprints/Camera/BP_Pawn.BP_Pawn_C|GetBothMouseButtonsPressed (Variables|Default|GetPawn)))
    (if (or (Variables|/Game/Blueprints/Camera/BP_Pawn.BP_Pawn_C|GetWKeyPressed (Variables|Default|GetPawn)) (Variables|/Game/Blueprints/Camera/BP_Pawn.BP_Pawn_C|GetSKeyPressed (Variables|Default|GetPawn)))
      (Pawn|Input|AddMovementInput (Variables|Default|GetPawn) (Math|Vector|GetForwardVector (Math|Rotator|MakeRotator 0.0 0.0 (.Yaw (Math|Rotator|BreakRotator (Pawn|GetControlRotation (Variables|Default|GetPawn) :!class /Script/Engine.Pawn))))) Scale false))))

(fn MoveUpKeyboard
  (params (Scale :type Float%20%28single-precision%29))
  (if (or (Variables|/Game/Blueprints/Camera/BP_Pawn.BP_Pawn_C|GetUpKeyPressed (Variables|Default|GetPawn)) (Variables|/Game/Blueprints/Camera/BP_Pawn.BP_Pawn_C|GetDownKeyPressed (Variables|Default|GetPawn)))
    (Pawn|Input|AddMovementInput (Variables|Default|GetPawn) "0, 0,1.000000" Scale false)))

(fn LookUpDownMouse
  (if (not (Variables|/Game/Blueprints/Camera/BP_Pawn.BP_Pawn_C|GetBothMouseButtonsPressed (Variables|Default|GetPawn)))
    (if (Variables|/Game/Blueprints/Camera/BP_Pawn.BP_Pawn_C|GetRightMouseButtonPressed (Variables|Default|GetPawn))
      (bind _result (Math|Float|NegateFloat (.LocationY (Game|Player|GetMousePosition (Game|GetPlayerController 0))))
        (:%20%20
          (Pawn|Input|AddControllerPitchInput (Variables|Default|GetPawn) _result))))))

(fn LookRightLeftMouse
  (if (not (Variables|/Game/Blueprints/Camera/BP_Pawn.BP_Pawn_C|GetBothMouseButtonsPressed (Variables|Default|GetPawn)))
    (if (or (Variables|/Game/Blueprints/Camera/BP_Pawn.BP_Pawn_C|GetRightMouseButtonPressed (Variables|Default|GetPawn)) (Variables|/Game/Blueprints/Camera/BP_Pawn.BP_Pawn_C|GetLeftMouseButtonPressed (Variables|Default|GetPawn)))
      (Pawn|Input|AddControllerYawInput (Variables|Default|GetPawn) (.LocationX (Game|Player|GetMousePosition (Game|GetPlayerController 0)))))))

(fn SetupBothMousesCheck
  (if (and (Variables|/Game/Blueprints/Camera/BP_Pawn.BP_Pawn_C|GetLeftMouseButtonPressed (Variables|Default|GetPawn)) (Variables|/Game/Blueprints/Camera/BP_Pawn.BP_Pawn_C|GetRightMouseButtonPressed (Variables|Default|GetPawn)))
    (bind _output_get (Variables|Default|SetPawn 0))
    (Variables|/Game/Blueprints/Camera/BP_Pawn.BP_Pawn_C|SetBothMouseButtonsPressed _output_get true)
    (else
      (bind _output_get_2 (Variables|Default|SetPawn 0))
      (Variables|/Game/Blueprints/Camera/BP_Pawn.BP_Pawn_C|SetBothMouseButtonsPressed _output_get_2 false))))

(fn SetupBothMouses
  (if (Variables|/Game/Blueprints/Camera/BP_Pawn.BP_Pawn_C|GetBothMouseButtonsPressed (Variables|Default|GetPawn))
    (Pawn|Input|AddMovementInput (Variables|Default|GetPawn) "0, 0,1.000000" (.LocationY (Game|Player|GetMousePosition (Game|GetPlayerController 0))) false)
    (Pawn|Input|AddMovementInput (Variables|Default|GetPawn) (Math|Vector|GetRightVector (Pawn|GetControlRotation (Variables|Default|GetPawn) :!class /Script/Engine.Pawn)) (.LocationX (Game|Player|GetMousePosition (Game|GetPlayerController 0))) false)))

(fn InitKeyboard
  (params (BP_Camera :type BP%20Pawn%20Object%20Reference))
  (Variables|Default|SetPawn BP_Camera))