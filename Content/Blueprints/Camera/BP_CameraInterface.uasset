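; Camera control interface that applies named movement actions to a character supplied through InitInterface, and can quit the simulation.
; On BeginPlay it builds a map of six directional move-camera command objects, following the Command pattern.
; AddAction and RemoveAction edit the active set, and Tick runs each active command with the character and a shared Factor.
; SetFactor adjusts that Factor incrementally, clamped between its minimum and maximum.
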(event EventBeginPlay
  (CallFunction|FillActions))

(event EventTick
  (params (DeltaSeconds :type Float%20%28single-precision%29))
  (CallFunction|ExecuteAction))

(fn QuitSimulation
  (Game|QuitGame (Game|GetPlayerController 0) "Quit" false)
  (Development|PrintString "Good bye"))

(fn InitInterface
  (params (Character :type BP%20Character%20Object%20Reference))
  (Variables|Default|SetCharacter Character))

(fn ExecuteAction
  (bind _values (Utilities|Map|Values (Variables|Action|GetActionsToExecute)))
  (for _array_element _values
    (Default|DoAction _array_element (Variables|Default|GetCharacter) (Variables|VelocityCamera|GetFactor))))

(fn FillActions
  (bind _returnvalue (Game|ConstructObjectfromClass "/Game/Blueprints/Camera/Actions/BP_MoveCameraUp.BP_MoveCameraUp_C" self))
  (Utilities|Map|Add (Variables|Action|GetActions) "Up" _returnvalue)
  (bind _returnvalue_2 (Game|ConstructObjectfromClass "/Game/Blueprints/Camera/Actions/BP_MoveCameraDown.BP_MoveCameraDown_C" self))
  (Utilities|Map|Add (Variables|Action|GetActions) "Down" _returnvalue_2)
  (bind _returnvalue_3 (Game|ConstructObjectfromClass "/Game/Blueprints/Camera/Actions/BP_MoveCameraForward.BP_MoveCameraForward_C" self))
  (Utilities|Map|Add (Variables|Action|GetActions) "Forward" _returnvalue_3)
  (bind _returnvalue_4 (Game|ConstructObjectfromClass "/Game/Blueprints/Camera/Actions/BP_MoveCameraBackward.BP_MoveCameraBackward_C" self))
  (Utilities|Map|Add (Variables|Action|GetActions) "Backward" _returnvalue_4)
  (bind _returnvalue_5 (Game|ConstructObjectfromClass "/Game/Blueprints/Camera/Actions/BP_MoveCameraLeft.BP_MoveCameraLeft_C" self))
  (Utilities|Map|Add (Variables|Action|GetActions) "Left" _returnvalue_5)
  (bind _returnvalue_6 (Game|ConstructObjectfromClass "/Game/Blueprints/Camera/Actions/BP_MoveCameraRight.BP_MoveCameraRight_C" self))
  (Utilities|Map|Add (Variables|Action|GetActions) "Right" _returnvalue_6))

(fn AddAction
  (params (ActionName :type String))
  (Utilities|Map|Add (Variables|Action|GetActionsToExecute) ActionName (.Value (Utilities|Map|Find (Variables|Action|GetActions) ActionName)))
  (return))

(fn SetFactor
  (params (FactorIncrease :type Float%20%28single-precision%29%20%28by%20ref%29))
  (if (< (+ FactorIncrease (Variables|VelocityCamera|GetFactor)) (Variables|VelocityCamera|GetMinFactor))
    (Variables|VelocityCamera|SetFactor (Variables|VelocityCamera|GetMinFactor))
    (return)
    (elif (> (+ FactorIncrease (Variables|VelocityCamera|GetFactor)) (Variables|VelocityCamera|GetMaxFactor))
      (Variables|VelocityCamera|SetFactor (Variables|VelocityCamera|GetMaxFactor))
      (return)
      (else
        (Variables|VelocityCamera|SetFactor (+ FactorIncrease (Variables|VelocityCamera|GetFactor)))
        (return)))))

(fn RemoveAction
  (params (Action :type String))
  (Utilities|Map|Remove (Variables|Action|GetActionsToExecute) Action)
  (return))