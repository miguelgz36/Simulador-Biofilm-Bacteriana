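; Central controller for a bacterial biofilm simulation, running it from main menu through loading, execution and report data.
; On BeginPlay it opens the menu with bacterium and block types read from DataTables.
; It spawns and drives a Surface actor, forwarding options, loading, pause and spawn-progress queries.
; StartSimulation either drops nutrient balls as presimulation or starts BacteriaManager colonization with the in-execution UI; GetReportData gathers that manager's results.
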(event EventBeginPlay
  (GUI|StartMainMenu))

(event EventTick
  (params (DeltaSeconds :type Float%20%28single-precision%29)))

(fn ConstructionScript)

(fn StartMainMenu
  (bind _returnvalue (Game|GetPlayerController 0))
  (bind _returnvalue_2 (UserInterface|CreateWidget "/Game/Blueprints/GUI/Start/MainMenuWidget.MainMenuWidget_C" _returnvalue "0.3" "20" "" "37"))
  (bind (_types _keys) (GUI|LoadBacteriumTypes))
  (bind (_types_2 _keys_2) (GUI|LoadBlockTypes))
  (Default|Init _returnvalue_2 (Variables|Simulation|GetOptions) _types _types_2 _keys _keys_2)
  (UserInterface|Viewport|AddtoViewport _returnvalue_2 0)
  (Input|SetInputModeUIOnly _returnvalue 0 "DoNotLock")
  (Variables|/Script/Engine.PlayerController|SetbShowMouseCursor _returnvalue true)
  (return))

(fn InitializeSurface
  (params (Options :type S%20Options%20Structure%20%28by%20ref%29))
  ;[1 1 1] Start loading calling all necesary functions
  (Variables|Simulation|SetOptions Options)
  (Default|Init (Variables|Surface|GetSurface) (Variables|Simulation|GetOptions))
  (bind _foundwidgets (Widget|GetAllWidgetsOfClass "/Game/Blueprints/GUI/Start/MainMenuWidget.MainMenuWidget_C" true))
  (Widget|RemovefromParent _foundwidgets)
  (return))

(fn SetPaused
  (params (Paused :type Boolean))
  (Default|SetPaused (Variables|Surface|GetSurface) Paused))

(fn GetSurface
  (return (Variables|Surface|GetSurface)))

(fn LoadBacteriumTypes
  (bind _outrownames (DataTable|GetDataTableRowNames "/Game/DataTables/DT_Bacterium.DT_Bacterium"))
  (for _array_element _outrownames
    (bind _returnvalue (Utilities|GetDataTableRow "/Game/DataTables/DT_Bacterium.DT_Bacterium" _array_element)
      (:then
        (Utilities|Array|Add (LocalVariables|GetBacteriumTypes) _returnvalue)
        (Utilities|Map|Add (LocalVariables|GetBacteriumKeys) (.Name (Utilities|Struct|BreakS_Bacterium _returnvalue)) (Utilities|String|ToString(Name) _array_element)))))
  (return (LocalVariables|GetBacteriumTypes) (LocalVariables|GetBacteriumKeys)))

(fn LoadBlockTypes
  (bind _outrownames (DataTable|GetDataTableRowNames "/Game/DataTables/DT_Block.DT_Block"))
  (for _array_element _outrownames
    (bind _returnvalue (Utilities|GetDataTableRow "/Game/DataTables/DT_Block.DT_Block" _array_element)
      (:then
        (Utilities|Array|Add (LocalVariables|GetBlocksTypes) _returnvalue)
        (Utilities|Map|Add (LocalVariables|GetBlocksKeys) (.Name (Utilities|Struct|BreakS_Block _returnvalue)) (Utilities|String|ToString(Name) _array_element)))))
  (return (LocalVariables|GetBlocksTypes) (LocalVariables|GetBlocksKeys)))

(fn StartSimulation
  ;[1 1 1] If presimulation was enabled, balls with nutrients start to falling on surface (when all are distributed bacteria colonization starts). If presimulation was disabled, bacteria colonization starts immediately.
  (if (.DoPresimulation (Utilities|Struct|BreakS_Options (Variables|Simulation|GetOptions)))
    (Default|ActivateBallsFalling (Variables|Surface|GetSurface))
    (else
      (bind _bacteriamanager (Default|GetBacteriaManager (Variables|Surface|GetSurface)))
      (Default|StartColonization _bacteriamanager)
      (GUI|StarinExecutionGUI))))

(fn GetNumberObjectstoSpawn
  (bind _options (Variables|Simulation|GetOptions))
  (bind _options_2 (Variables|Simulation|GetOptions))
  (bind (_bacteria _surface _factornutrientupdatepersize _dopresimulation _presimulationgranularity _blocksperside _temperature _initialenergylevel _maximumenergylevel _nutrientlevelthresholdtomove _minimumenergylevel _energyspenttomove _maximummovementattempts _minimumnutrientlevel _unitsradiustomove _initialnumberbacteriainmemory) (Utilities|Struct|BreakS_Options _options))
  (bind (_bacteria_2 _surface_2 _factornutrientupdatepersize_2 _dopresimulation_2 _presimulationgranularity_2 _blocksperside_2 _temperature_2 _initialenergylevel_2 _maximumenergylevel_2 _nutrientlevelthresholdtomove_2 _minimumenergylevel_2 _energyspenttomove_2 _maximummovementattempts_2 _minimumnutrientlevel_2 _unitsradiustomove_2 _initialnumberbacteriainmemory_2) (Utilities|Struct|BreakS_Options _options_2))
  (bind _returnvalue (* _presimulationgranularity _presimulationgranularity))
  (bind _returnvalue_2 (* _blocksperside _blocksperside))
  (bind _returnvalue_3 (* _blocksperside_2 _blocksperside_2))
  (bind _returnvalue_4 (* _returnvalue _returnvalue_2))
  (if _dopresimulation_2
    (return (+ (+ _returnvalue_4 _returnvalue_2) _initialnumberbacteriainmemory) _returnvalue_2 _returnvalue_4 _initialnumberbacteriainmemory)
    (else
      (return (+ _returnvalue_3 _initialnumberbacteriainmemory_2) _returnvalue_3 0 _initialnumberbacteriainmemory_2))))

(fn CreateHomogeneusSurface
  (bind _returnvalue (Game|SpawnActorfromClass "/Game/Blueprints/Surface/Surfaces/BP_Surface_Homogeneous.BP_Surface_Homogeneous_C" (Math|Transform|MakeTransform "0, 0, 0") "AlwaysSpawn" 0 0))
  (Variables|Surface|SetSurface _returnvalue))

(fn SetOptions
  (params (Options :type S%20Options%20Structure%20%28by%20ref%29))
  (Variables|Simulation|SetOptions Options))

(fn GetNumberObjectsSpawned
  (bind _numberobjectsspawned (Default|GetNumberObjectsSpawned (Variables|Surface|GetSurface)))
  (return _numberobjectsspawned))

(fn GetReportData
  (bind _bacteriamanager (Default|GetBacteriaManager (Variables|Surface|GetSurface)))
  (bind _maxbiofilmarea (Default|GetMaxBiofilmArea _bacteriamanager))
  (bind _maxbacteriacounter (Default|GetMaxBacteriaCounter _bacteriamanager))
  (bind _bacteriapositions (Default|GetBacteriaPositionsonSurface _bacteriamanager))
  (bind _mapbounds (Default|GetMapBounds (Variables|Surface|GetSurface)))
  (bind _datapertime (Default|GetBacteriaDataPerTime _bacteriamanager))
  (return _datapertime (Variables|Simulation|GetOptions) _mapbounds _bacteriapositions _maxbacteriacounter _maxbiofilmarea))

(fn StartLoading
  (Default|LoadObjects (Variables|Surface|GetSurface)))

(fn StarinExecutionGUI
  (bind _returnvalue (Game|GetPlayerController 0))
  ;[1 1 1] Generate the UI required elements to start the simulation
  (bind _returnvalue_2 (UserInterface|CreateWidget "/Game/Blueprints/GUI/Simulation/InExecution.InExecution_C" _returnvalue))
  (Default|Init _returnvalue_2)
  (UserInterface|Viewport|AddtoViewport _returnvalue_2 0)
  (Input|SetInputModeGameandUI _returnvalue _returnvalue_2 "DoNotLock" true)
  (Variables|/Script/Engine.PlayerController|SetbShowMouseCursor _returnvalue true))