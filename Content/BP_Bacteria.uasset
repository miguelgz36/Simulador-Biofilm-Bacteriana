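; BP_Bacteria is an actor simulating a bacterium that feeds and reproduces by binary fission.
; A looping timer started on BeginPlay runs LifeCycle at a fixed interval, without using Tick.
; Each cycle updates EnergyLevel through ConsumeNutrients from the available nutrient.
; At maximum energy, it calls BinaryFission with its own class, itself as owner and its dimensions, then resets energy to zero.
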(event Custom|CustomEvent_0
  (CallFunction|LifeCycle))

(event EventBeginPlay
  (Utilities|Time|SetTimerbyEvent (delegate Custom|CustomEvent_0) 2.0 true 2.0))

(event Collision|EventActorBeginOverlap
  (params (OtherActor :type Actor%20Object%20Reference)))

(event EventTick
  (params (DeltaSeconds :type Float%20%28single-precision%29)))

(fn ConstructionScript)

(fn LifeCycle
  (bind _returnvalue (Class|ConsumeNutrients|GetNutrients (Variables|Default|GetConsumeNutrients) (Variables|Default|GetAvailableNutrient) (Variables|Default|GetEnergyLevel)))
  (Variables|Default|SetEnergyLevel _returnvalue)
  (if (>= (Variables|Default|GetEnergyLevel) (Variables|Default|GetMaximumEnergyLevel))
    (Class|BinaryFission|DoBinaryFission (Variables|Default|GetBinaryFission) "BP_Bacteria_C" self (Variables|Default|GetLength) (Variables|Default|GetWidth))
    (Variables|Default|SetEnergyLevel 0.0)))